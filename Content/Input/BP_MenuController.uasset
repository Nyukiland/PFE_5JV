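; BP_MenuController is the menu player controller, opening the main menu widget, handling trigger input and loading the game level on start.
; Analog triggers, with Z and C as key alternatives, broadcast values and become pressed states past a threshold.
; A short real-time buffer, resolved on Tick, separates single presses from a both-trigger chord before firing Left, Right or Both dispatchers.
; Options open and close events are empty, their widget logic disconnected.
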(event `EvaluateInput`
  ; Trigger behaviours in menus
  (if (and (`self.TriggerLeft`) (`self.TriggerRight`))
    (set `self.OnBufferInput` false)
    (`self.TriggerTriggeringTheTriggerBoth`)
    (else
      (set `self.OnBufferInput` true)
      (set `self.TargetRealtime` (+ (`GameplayStatics.GetRealTimeSeconds`) 0.05)))))

(event `EnhancedInput|/Game/Input/IA_LeftTrigger`
  (params (ActionValue :type "Float (double-precision)") (ElapsedSeconds :type "Float (double-precision)") (TriggeredSeconds :type "Float (double-precision)") (InputAction :type "InputAction Object Reference" :default "/Game/Input/IA_LeftTrigger.IA_LeftTrigger"))
  (bind _triggerleft (`self.TriggerLeft`))
  ; Trigger behaviours in menus
  (:`Triggered`
    (`self.InputLeftValue` ActionValue)
    (if (> ActionValue 0.5)
      (if (not _triggerleft)
        (set `self.TriggerLeft` true :!label _label)
        (`self.EvaluateInput`))
      (elif _triggerleft
        (set `self.TriggerLeft` false :!label _label_2))))
  (:`Canceled`
    (goto _label_2))
  (:`Completed`
    (goto _label_2)))

(event `self.ReceiveBeginPlay`
  (`EnhancedInputSubsystemInterface.AddMappingContext` (pcsubsystem `EnhancedInputLocalPlayerSubsystem` (`GameplayStatics.GetPlayerController` 0)) "/Game/Input/IMC_InputMap.IMC_InputMap" 0 (struct)))

(event `Key|Z` :consume false
  (params (Key :type "Key Structure"))
  ; Trigger behaviours in menus
  (:`Pressed`
    (goto _label))
  (:`Released`
    (goto _label_2)))

(event `FirstSetup`
  (`WidgetBlueprintLibrary.SetInputMode_GameOnly` self)
  (set `self.bShowMouseCursor` false))

(event `self.ReceiveTick`
  (params (DeltaSeconds :type "Float (single-precision)"))
  ; Trigger behaviours in menus
  (if (and (`self.OnBufferInput`) (>= (`GameplayStatics.GetRealTimeSeconds`) (`self.TargetRealtime`)))
    (if (`self.TriggerLeft`)
      (`self.TriggerTriggeringTheTriggerLeft`)
      (set `self.OnBufferInput` false)
      (elif (`self.TriggerRight`)
        (`self.TriggerTriggeringTheTriggerRight`)
        (set `self.OnBufferInput` false)))))

(event `OpenMainMenu`
  (bind _returnvalue (`|CreateWidget` "/Game/Blueprint/UI/UW_MainMenu.UW_MainMenu_C" self))
  (`UserWidget.AddToViewport` _returnvalue 0)
  (set `self.MainMenuRef` _returnvalue)
  (`/Game/Blueprint/UI/UW_MainMenu.SetupControls` _returnvalue)
  (`/Game/Blueprint/UI/UW_MainMenu.StartMainMenuAnim` _returnvalue))

(event `EnhancedInput|/Game/Input/IA_RightTrigger`
  (params (ActionValue :type "Float (double-precision)") (ElapsedSeconds :type "Float (double-precision)") (TriggeredSeconds :type "Float (double-precision)") (InputAction :type "InputAction Object Reference" :default "/Game/Input/IA_RightTrigger.IA_RightTrigger"))
  (bind _triggerright (`self.TriggerRight`))
  ; Trigger behaviours in menus
  (:`Triggered`
    (`self.InputRightValue` ActionValue)
    (if (> ActionValue 0.5)
      (if (not _triggerright)
        (set `self.TriggerRight` true :!label _label_3)
        (`self.EvaluateInput`))
      (elif _triggerright
        (set `self.TriggerRight` false :!label _label_4))))
  (:`Canceled`
    (goto _label_4))
  (:`Completed`
    (goto _label_4)))

(event `OpenOptions`)

(event `Key|C` :consume false
  (params (Key :type "Key Structure"))
  ; Trigger behaviours in menus
  (:`Pressed`
    (goto _label_3))
  (:`Released`
    (goto _label_4)))

(event `CloseOptions`)

(event `StartGame`
  (params (`Main Menu Ref` :type "/Game/Blueprint/UI/UW_MainMenu Object Reference"))
  (`Widget.RemoveFromParent` `Main Menu Ref`)
  (`GameplayStatics.OpenLevelBySoftObjectPtr` "/Game/Level/TestTytyne/L_Game.L_Game"))

(fn `UserConstructionScript`)