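; BP_Controller turns left and right trigger input into left, right or both-trigger calls for menu behaviours.
; Enhanced Input actions, with Z and C keys as alternatives, set held flags using a half-press threshold and evaluate on each new press.
; Holding both fires immediately, while a single press starts a short real-time buffer that Tick resolves to whichever trigger is still held, favouring left.
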(event `EvaluateInput`
  ; Trigger behaviours in menus
  (if (and (`self.TriggerLeft`) (`self.TriggerRight`))
    (set `self.OnBufferInput` false)
    (`self.BothTrigger`)
    (else
      (set `self.OnBufferInput` true)
      (set `self.TargetRealtime` (+ (`GameplayStatics.GetRealTimeSeconds`) 0.05)))))

(event `EnhancedInput|/Game/Input/IA_LeftTrigger`
  (params (ActionValue :type "Float (double-precision)") (ElapsedSeconds :type "Float (double-precision)") (TriggeredSeconds :type "Float (double-precision)") (InputAction :type "InputAction Object Reference" :default "/Game/Input/IA_LeftTrigger.IA_LeftTrigger"))
  (bind _triggerleft (`self.TriggerLeft`))
  ; Trigger behaviours in menus
  (:`Triggered`
    (if (> ActionValue 0.5)
      (if (not _triggerleft)
        (set `self.TriggerLeft` true :!label _label)
        (`self.EvaluateInput`))
      (elif _triggerleft
        (set `self.TriggerLeft` false :!label _label_2))))
  (:`Canceled`
    (goto _label_2))
  (:`Completed`
    (goto _label_2)))

(event `Key|Z` :consume false
  (params (Key :type "Key Structure"))
  ; Trigger behaviours in menus
  (:`Pressed`
    (goto _label))
  (:`Released`
    (goto _label_2)))

(event `self.ReceiveTick`
  (params (DeltaSeconds :type "Float (single-precision)"))
  ; Trigger behaviours in menus
  (if (and (`self.OnBufferInput`) (>= (`GameplayStatics.GetRealTimeSeconds`) (`self.TargetRealtime`)))
    (if (`self.TriggerLeft`)
      (`self.LeftTrigger`)
      (set `self.OnBufferInput` false)
      (elif (`self.TriggerRight`)
        (`self.RightTrigger`)
        (set `self.OnBufferInput` false)))))

(event `EnhancedInput|/Game/Input/IA_RightTrigger`
  (params (ActionValue :type "Float (double-precision)") (ElapsedSeconds :type "Float (double-precision)") (TriggeredSeconds :type "Float (double-precision)") (InputAction :type "InputAction Object Reference" :default "/Game/Input/IA_RightTrigger.IA_RightTrigger"))
  (bind _triggerright (`self.TriggerRight`))
  ; Trigger behaviours in menus
  (:`Triggered`
    (if (> ActionValue 0.5)
      (if (not _triggerright)
        (set `self.TriggerRight` true :!label _label_3)
        (`self.EvaluateInput`))
      (elif _triggerright
        (set `self.TriggerRight` false :!label _label_4))))
  (:`Canceled`
    (goto _label_4))
  (:`Completed`
    (goto _label_4)))

(event `Key|C` :consume false
  (params (Key :type "Key Structure"))
  ; Trigger behaviours in menus
  (:`Pressed`
    (goto _label_3))
  (:`Released`
    (goto _label_4)))

(fn `UserConstructionScript`)