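; BP_Ronce is a bramble mesh actor that animates the "Offset" scalar parameter on its static mesh's materials.
; Each Tick checks ActiveAnimation: true plays a timeline lerping the offset from MatStart to MatStop, false plays a second timeline lerping it back.
; Both timelines use Play rather than Play from Start and are never reversed or reset here.
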(event `self.ReceiveTick`
  (params (DeltaSeconds :type "Float (single-precision)"))
  (bind _staticmesh (`self.StaticMesh`))
  (if (`self.Active_animation`)
    (bind (_direction _time) (`Timeline|Timeline`)
      (:`Update`
        (`MeshComponent.SetScalarParameterValueOnMaterials` _staticmesh "Offset" (`KismetMathLibrary.Lerp` (`self.matStart`) (`self.matStop`) _time))))
    (else
      (bind (_direction_2 _time_2) (`Timeline|Timeline_0`)
        (:`Update`
          (`MeshComponent.SetScalarParameterValueOnMaterials` _staticmesh "Offset" (`KismetMathLibrary.Lerp` (`self.matStop`) (`self.matStart`) _time_2)))))))

(fn `UserConstructionScript`)