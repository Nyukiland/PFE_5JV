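; Level-design action Blueprint that gradually scales the actors in its ActorList by an additive offset over a set duration.
; DoAction calls the parent, records each actor's current scale and its target of that scale plus ScaleOffset, then starts LoopTime.
; LoopTime advances a clamped timer, lerps each scale by elapsed time over Duration, and re-triggers itself through next-tick delays until Time reaches Duration.
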(event `LoopTime`
  (bind _duration (`self.Duration`))
  (`PFMathHelper.IncrementFloat` (`self.time`) (`GameplayStatics.GetWorldDeltaSeconds`))
  (bind _returnvalue (`PFMathHelper.ClampFloatByRef` (`self.time`) 0.0 _duration))
  (for (_array_element _array_index) (`self.ActorList`)
    (`self.SetActorScale3D` _array_element (`KismetMathLibrary.VLerp` (`|GetArrayItem` (`self.startScale`) _array_index) (`|GetArrayItem` (`self.EndScale`) _array_index) (/ _returnvalue _duration)))
    (if (not (== (`self.time`) (`self.Duration`)))
      (`KismetSystemLibrary.DelayUntilNextTick`)
      (`self.LoopTime`))))

(fn `DoAction`
  (`parent.DoAction`)
  (`KismetArrayLibrary.Array_Clear` (`self.startScale`))
  (`KismetArrayLibrary.Array_Clear` (`self.EndScale`))
  (for _array_element (`self.ActorList`)
    (bind _returnvalue (`self.GetActorScale3D` _array_element))
    (`KismetArrayLibrary.Array_Add` (`self.startScale`) _returnvalue)
    (`KismetArrayLibrary.Array_Add` (`self.EndScale`) (+ _returnvalue (`self.ScaleOffset`))))
  (`self.LoopTime`))

(fn `UserConstructionScript`
  (`parent.UserConstructionScript`))