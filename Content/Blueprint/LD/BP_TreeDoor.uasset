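; BP_TreeDoor is a door actor that opens when its inherited DoAction runs.
; DoAction calls the parent, disables StaticMesh collision and sets the "Offset" material parameter between Close and Open, so the visual change is material-driven.
; The blend alpha is frame delta times Time, clamped and evaluated once per call, with no timeline or tick in this Blueprint.
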(fn `DoAction`
  (bind _staticmesh (`self.StaticMesh`))
  (`parent.DoAction`)
  (`PrimitiveComponent.SetCollisionEnabled` _staticmesh "NoCollision")
  (`MeshComponent.SetScalarParameterValueOnMaterials` _staticmesh "Offset" (`KismetMathLibrary.Lerp` (`self.Close`) (`self.Open`) (`KismetMathLibrary.FClamp` (* (`GameplayStatics.GetWorldDeltaSeconds`) (`self.Time`))))))

(fn `UserConstructionScript`)