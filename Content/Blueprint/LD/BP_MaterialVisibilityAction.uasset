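; Level-design action that fades the "Visibility" material parameter on chosen static meshes from 0 toward 1 over a set Timer.
; DoAction extends its parent, creating dynamic material instances for each mesh and material index pair in the Meshes map.
; The Loop event, started as each instance is added, accumulates delta time, writes Time/Timer to every instance and re-calls itself through next-tick delays instead of using Tick.
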(event `self.ReceiveTick`
  (params (DeltaSeconds :type "Float (single-precision)")))

(event `Loop`
  (set `self.Time` (+ (`self.Time`) (`GameplayStatics.GetWorldDeltaSeconds`)))
  (if (>= (`self.Timer`) (`self.Time`))
    (for _array_element (`self.MaterialList`)
      (`MaterialInstanceDynamic.SetScalarParameterValue` _array_element "Visibility" (/ (`self.Time`) (`self.Timer`)))
      (`KismetSystemLibrary.DelayUntilNextTick`)
      (`self.Loop`))))

(fn `DoAction`
  (`parent.DoAction`)
  (bind (_keypin _valuepin) (`|MapForEach` (`self.Meshes`))
    (:`then`
      (bind _staticmeshcomponent (`StaticMeshActor.StaticMeshComponent` _keypin))
      (bind _returnvalue (`PrimitiveComponent.CreateDynamicMaterialInstance` _staticmeshcomponent _valuepin (`|GetArrayItem` (`MeshComponent.GetMaterials` _staticmeshcomponent) _valuepin) "None"))
      (`KismetArrayLibrary.Array_Add` (`self.MaterialList`) _returnvalue)
      (`self.Loop`))))

(fn `UserConstructionScript`
  (`parent.UserConstructionScript`))