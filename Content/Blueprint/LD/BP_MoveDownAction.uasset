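; BP_MoveDownAction is a level design action that smoothly moves its own actor by MoveOffset over Duration.
; DoAction calls the parent, captures the current location as StartPos, derives EndPos from the offset, then starts LoopTime.
; LoopTime advances a clamped timer by delta seconds and linearly interpolates the location without sweep.
; It re-calls itself through DelayUntilNextTick until the timer equals Duration, avoiding Event Tick and Timelines.
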(event `LoopTime`
  (bind _duration (`self.Duration`))
  (`PFMathHelper.IncrementFloat` (`self.time`) (`GameplayStatics.GetWorldDeltaSeconds`))
  (bind _returnvalue (`PFMathHelper.ClampFloatByRef` (`self.time`) 0.0 _duration))
  (`self.K2_SetActorLocation` (`KismetMathLibrary.VLerp` (`self.startPos`) (`self.endPos`) (/ _returnvalue _duration)))
  (if (not (== (`self.time`) (`self.Duration`)))
    (`KismetSystemLibrary.DelayUntilNextTick`)
    (`self.LoopTime`)))

(fn `DoAction`
  (`parent.DoAction`)
  (bind _output_get (set `self.startPos` (`self.K2_GetActorLocation`)))
  (set `self.endPos` (+ _output_get (`self.MoveOffset`)))
  (`self.LoopTime`))

(fn `UserConstructionScript`
  (`parent.UserConstructionScript`))