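; Player visual resource component that spawns the visual actor on the bird root and drives movement and flower effects.
; Tick writes player position and speed-line intensity to a post-process parameter collection, while getters expose speed-remapped line values and drift state.
; Flower color changes recolor or disable petal Niagara; water particles restart on demand.
; A hidden key combo (Right Ctrl, Right Shift presses, letter) swaps the visual for jet, ball, dragon and other forms.
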(event `self.ComponentInit`
  (params (ownerObj :type "PFPlayerCharacter Object Reference"))
  (`parent.ComponentInit` ownerObj)
  (`self.SpawnVisu` (`self.InitialVisuPtr`))
  (bind _returnvalue (`PFPlayerCharacter.GetStateComponent` (`self.Owner`) "/Game/Blueprint/Player/Resource/Physic/BP_PhysicResource.BP_PhysicResource_C"))
  (set `self.PhysicPtr` _returnvalue)
  (bind _returnvalue_2 (`PFPlayerCharacter.GetStateComponent` (`self.Owner`) "/Game/Blueprint/Player/Ability/Turn/BP_TurnAbility.BP_TurnAbility_C"))
  (set `self.TurnPtr` _returnvalue_2)
  (bind _returnvalue_3 (`PFPlayerCharacter.GetStateComponent` (`self.Owner`) "/Game/Blueprint/Player/Resource/FlowerSpawner/BP_FlowerSpawnerResource.BP_FlowerSpawnerResource_C"))
  (bind _output_get (set `self.FlowerResource` _returnvalue_3))
  (add `PFFlowerSpawnerResource.OnFlowerColorChangeDelegate` _output_get (delegate `OnFlowerColorChange`))
  (`KismetSystemLibrary.DelayUntilNextTick`)
  (`KismetSystemLibrary.DelayUntilNextTick`)
  (`self.Deactivate` (`self.PetalNiagara`))
  (`self.Deactivate` (`self.WaterNiagara`)))

(event `OnFlowerColorChange`
  (params (FlowerColor :type "EPFFlowerColor Enum" :default "EPFFC_None"))
  (`self.ChangeParticleColor` FlowerColor))

(event `self.ComponentTick`
  (params (deltaTime :type "Float (single-precision)"))
  (bind (_speedlineintensityremap_x _speedlineintensityremap_y _speedlineintensityremap_z _speedlineintensityremap_w) (`KismetMathLibrary.BreakVector4` (`self.SpeedLineIntensityRemap`)))
  (`parent.ComponentTick` deltaTime)
  (`KismetMaterialLibrary.SetVectorParameterValue` "/Game/Materials/POST_PROCESS/MParameter_PostPro.MParameter_PostPro" "PlayerXY" (`KismetMathLibrary.Conv_VectorToLinearColor` (`SceneComponent.K2_GetComponentLocation` (`self.BirdVisualRootPtr_`))))
  (bind _returnvalue (`PFMathHelper.RemapClamped` (`KismetMathLibrary.VSize` (`PFPhysicResource.CurrentForwardVelocity_` (`self.PhysicPtr`))) _speedlineintensityremap_x _speedlineintensityremap_y _speedlineintensityremap_z _speedlineintensityremap_w))
  (`KismetMaterialLibrary.SetScalarParameterValue` "/Game/Materials/POST_PROCESS/MParameter_PostPro.MParameter_PostPro" "SpeedLineIntensity" _returnvalue))

(event `Key|A`
  (params (Key :type "Key Structure"))
  (:`Pressed`
    (`self.TryChangeVisu` "/Game/Blueprint/Player/PlayerVisu/BP_Jet.BP_Jet_C")))

(event `Key|F`
  (params (Key :type "Key Structure")))

(event `Key|K`
  (params (Key :type "Key Structure")))

(event `Key|P`
  (params (Key :type "Key Structure")))

(event `Key|U`
  (params (Key :type "Key Structure")))

(event `Key|Z`
  (params (Key :type "Key Structure")))

(event `Key|B`
  (params (Key :type "Key Structure"))
  (:`Pressed`
    (`self.TryChangeVisu` "/Game/Blueprint/Player/PlayerVisu/BP_Ball.BP_Ball_C")))

(event `Key|G`
  (params (Key :type "Key Structure")))

(event `Key|L`
  (params (Key :type "Key Structure")))

(event `Key|Q`
  (params (Key :type "Key Structure")))

(event `Key|V`
  (params (Key :type "Key Structure")))

(event `Key|RightShift`
  (params (Key :type "Key Structure"))
  (:`Pressed`
    (`PFMathHelper.IncrementInt` (`self.ShiftCount`) 1)
    (set `self.TimerShiftCount` 0.0))
  (:`Released`
    (if (>= (`self.TimerShiftCount`) 1.0)
      (set `self.ShiftCount` 0))))

(event `Key|C`
  (params (Key :type "Key Structure")))

(event `Key|H`
  (params (Key :type "Key Structure")))

(event `Key|M`
  (params (Key :type "Key Structure"))
  (:`Pressed`
    (`self.TryChangeVisu` "/Game/Blueprint/Player/PlayerVisu/BP_Manta.BP_Manta_C")))

(event `Key|R`
  (params (Key :type "Key Structure"))
  (:`Pressed`
    (`self.TryChangeVisu` "/Game/Blueprint/Player/PlayerVisu/BP_Roti.BP_Roti_C")))

(event `Key|W`
  (params (Key :type "Key Structure")))

(event `Key|D`
  (params (Key :type "Key Structure"))
  (:`Pressed`
    (`self.TryChangeVisu` "/Game/Blueprint/Player/PlayerVisu/BP_Dragon.BP_Dragon_C")))

(event `Key|I`
  (params (Key :type "Key Structure")))

(event `Key|N`
  (params (Key :type "Key Structure")))

(event `Key|S`
  (params (Key :type "Key Structure")))

(event `Key|X`
  (params (Key :type "Key Structure")))

(event `Key|RightControl`
  (params (Key :type "Key Structure"))
  (:`Pressed`
    (set `self.ValidForCount` true))
  (:`Released`
    (set `self.ValidForCount` false)))

(event `Key|E`
  (params (Key :type "Key Structure")))

(event `Key|J`
  (params (Key :type "Key Structure")))

(event `Key|O`
  (params (Key :type "Key Structure"))
  (:`Pressed`
    (`self.TryChangeVisu` "/Game/Blueprint/Player/PlayerVisu/BP_Bird.BP_Bird_C")))

(event `Key|T`
  (params (Key :type "Key Structure")))

(event `Key|Y`
  (params (Key :type "Key Structure")))

(fn `CallWaterParticle`
  (`/Engine/EditorBlueprintResources/StandardMacros.IsValid` (`self.WaterNiagara`)
    (:`Is Valid`
      (`NiagaraComponent.ResetSystem` (`self.WaterNiagara`)))
    (:`Is Not Valid`
      (`KismetSystemLibrary.PrintString` "VisualResource / Water effect not valid"))))

(fn `ChangeParticleColor`
  (params (FlowerColor :type "EPFFlowerColor Enum" :default "EPFFC_None"))
  (locals (ColorValue :type "LinearColor Structure"))
  (bind _colorvalue (`local.ColorValue`))
  (bind _petalniagara (`self.PetalNiagara`))
  (`/Engine/EditorBlueprintResources/StandardMacros.IsValid` (`self.PetalNiagara`)
    (:`Is Valid`
      (bind (_colorvalue_2 _returnvalue) (`PFFlowerSpawnerResource.TryGetFlowerColorFromEnum` (`self.FlowerResource`) FlowerColor))
      (set `local.ColorValue` _colorvalue_2)
      (if _returnvalue
        (if (not (`self.IsActive` _petalniagara))
          (`self.Activate` _petalniagara true))
        (`NiagaraComponent.SetVariableLinearColor` (`self.PetalNiagara`) "ParticleColor" _colorvalue)
        (`KismetSystemLibrary.PrintString` (`KismetStringLibrary.Conv_ColorToString` _colorvalue))
        (else
          (`self.Deactivate` (`self.PetalNiagara`)))))
    (:`Is Not Valid`
      (`KismetSystemLibrary.PrintString` "VisualResource / Petal effect not valid"))))

(fn `CountChecker`
  (params (DeltaTime :type "Float (double-precision)"))
  (if (and (`self.ValidForCount`) (>= (`self.ShiftCount`) 1))
    (bind _returnvalue (`PFMathHelper.IncrementFloat` (`self.TimerShiftCount`) (`local.DeltaTime`)))
    (if (not (and (>= _returnvalue 1.0) (>= (`self.ShiftCount`) 3)))
      (set `self.ShiftCount` 0))))

(fn `GetAlphaLineValue`
  (returns (Value :type "Float (double-precision)"))
  (bind (_alphalineremap_x _alphalineremap_y _alphalineremap_z _alphalineremap_w) (`KismetMathLibrary.BreakVector4` (`self.AlphaLineRemap`)))
  (bind _returnvalue (`PFMathHelper.RemapClamped` (`KismetMathLibrary.VSize` (`PFPhysicResource.CurrentForwardVelocity_` (`self.PhysicPtr`))) _alphalineremap_x _alphalineremap_y _alphalineremap_z _alphalineremap_w))
  (return _returnvalue))

(fn `GetDriftingState`
  (returns (value :type Boolean))
  (return (`PFTurnAbility.bIsDrifting` (`self.TurnPtr`))))

(fn `GetSpeedLineValue`
  (returns (value :type "Float (double-precision)"))
  (bind (_speedlineremap_x _speedlineremap_y _speedlineremap_z _speedlineremap_w) (`KismetMathLibrary.BreakVector4` (`self.SpeedLineRemap`)))
  (bind _returnvalue (`PFMathHelper.RemapClamped` (`KismetMathLibrary.VSize` (`PFPhysicResource.CurrentForwardVelocity_` (`self.PhysicPtr`))) _speedlineremap_x _speedlineremap_y _speedlineremap_z _speedlineremap_w))
  (return _returnvalue))

(fn `SpawnVisu`
  (params (SpawnClass :type "/Game/Blueprint/Player/PlayerVisu/BP_VisuParent Class Reference"))
  (`/Engine/EditorBlueprintResources/StandardMacros.IsValid` (`self.CurrentVisuPtr`)
    (:`Is Valid`
      (`Actor.K2_DestroyActor` (`self.CurrentVisuPtr`)))
    (:`Is Not Valid`
      _))
  (bind _returnvalue (`|SpawnActorFromClass` (`local.SpawnClass`) (`SceneComponent.K2_GetComponentToWorld` (`self.BirdVisualRootPtr_`)) "AlwaysSpawn" "MultiplyWithRoot" (`self.Owner`) null))
  (bind _output_get (set `self.CurrentVisuPtr` _returnvalue))
  (`Actor.K2_AttachToComponent` _output_get (`self.BirdVisualRootPtr_`) "None" "SnapToTarget" "SnapToTarget" "SnapToTarget" false)
  (`/Game/Blueprint/Player/PlayerVisu/BP_VisuParent.SetOwnerParent` (`self.CurrentVisuPtr`) (`self.Owner`)))

(fn `TryChangeVisu`
  (params (Visu :type "/Game/Blueprint/Player/PlayerVisu/BP_VisuParent Class Reference"))
  (if (`KismetSystemLibrary.IsValidClass` Visu)
    (if (and (`self.ValidForCount`) (>= (`self.ShiftCount`) 3))
      (if (!= (`GameplayStatics.GetObjectClass` (`self.CurrentVisuPtr`)) (`local.Visu`))
        (`self.SpawnVisu` (`local.Visu`))))))