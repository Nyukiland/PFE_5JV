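; Player sound component that drives FMOD wind, music and one-shot sounds for wingbeats, dives and flower blooms.
; On init it starts wind, music and cave snapshot instances, binds the wingbeat event and caches the physics and proximity resources.
; Each tick it feeds smoothed speed and proximity values into wind and music parameters, with speed rising instantly and decaying gradually.
; A clamped counter plays or stops the cave snapshot.
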(event `self.ComponentInit`
  (params (ownerObj :type "PFPlayerCharacter Object Reference"))
  (`parent.ComponentInit` ownerObj)
  (bind _returnvalue (`PFPlayerCharacter.GetStateComponent` (`self.Owner`) "/Game/Blueprint/Player/Ability/WingBeat/BP_WingbeatAbility.BP_WingbeatAbility_C"))
  (add `PFWingBeatAbility.OnWingBeatCalled` _returnvalue (delegate `On WingBeat Sound`))
  (bind _returnvalue_2 (`PFPlayerCharacter.GetStateComponent` (`self.Owner`) "/Game/Blueprint/Player/Resource/Physic/BP_PhysicResource.BP_PhysicResource_C"))
  (set `self.PhysicResource` _returnvalue_2)
  (bind _returnvalue_3 (`PFPlayerCharacter.GetStateComponent` (`self.Owner`) "/Game/Blueprint/Player/Resource/Proximity/BP_ProximityResource.BP_ProximityResource_C"))
  (set `self.Proximity` _returnvalue_3)
  (bind _returnvalue_4 (`FMODBlueprintStatics.PlayEvent2D` (`self.Wind`)))
  (set `self.WindInstance` _returnvalue_4)
  (bind _returnvalue_5 (`FMODBlueprintStatics.PlayEvent2D` (`self.Music`)))
  (set `self.MusicInstance` _returnvalue_5)
  (bind _returnvalue_6 (`FMODBlueprintStatics.PlayEvent2D` (`self.CaveSnapshot`)))
  (set `self.CaveSnapshotInstance` _returnvalue_6))

(event `On WingBeat Sound`
  (`FMODBlueprintStatics.PlayEvent2D` (`self.Flap`)))

(event `self.ComponentTick`
  (params (deltaTime :type "Float (single-precision)"))
  (`parent.ComponentTick` deltaTime)
  (`self.SpeedVariation` deltaTime)
  (`self.GroundVariation` deltaTime))

(fn `CallDive`
  (`FMODBlueprintStatics.PlayEvent2D` (`self.Dive`)))

(fn `CallDiveExit`
  (`FMODBlueprintStatics.PlayEvent2D` (`self.DiveExit`)))

(fn `CallFlowerBloom`
  (`FMODBlueprintStatics.PlayEvent2D` (`self.FlowerBloom`)))

(fn `GroundVariation`
  (params (deltaTime :type "Float (double-precision)"))
  (bind _returnvalue (* (`self.ClosestDelayed`) 100.0))
  (if (< (`PFProximityResource.GetClosestDistancePercentage` (`self.Proximity`)) (`self.ClosestDelayed`))
    (`PFMathHelper.IncrementFloat` (`self.ClosestDelayed`) (* (`self.ClosestSlowSpeedIn`) (`local.deltaTime`)))
    (else
      (`PFMathHelper.DecrementFloat` (`self.ClosestDelayed`) (* (`self.ClosestSlowSpeedOut`) (`local.deltaTime`)))))
  (`PFMathHelper.ClampFloatByRef` (`self.ClosestDelayed`) 0.0 1.0)
  (`FMODBlueprintStatics.EventInstanceSetParameter` (`self.MusicInstance`) "Heal" _returnvalue)
  (`FMODBlueprintStatics.EventInstanceSetParameter` (`self.WindInstance`) "Low_Flying" _returnvalue))

(fn `SetCaveAmbiance`
  (params (inCaveCount :type Integer))
  (`PFMathHelper.IncrementInt` (`self.CaveCount`) inCaveCount)
  (bind _returnvalue (`PFMathHelper.ClampIntByRef` (`self.CaveCount`) 0 10000))
  (if (<= _returnvalue 0)
    (`FMODBlueprintStatics.EventInstanceStop` (`self.CaveSnapshotInstance`))
    (else
      (`FMODBlueprintStatics.EventInstancePlay` (`self.CaveSnapshotInstance`)))))

(fn `SpeedVariation`
  (params (deltaTime :type "Float (double-precision)"))
  (bind _returnvalue (* (`self.SpeedDelayed`) 100.0))
  (if (<= (`self.SpeedDelayed`) (`PFPhysicResource.GetForwardVelocityPercentage` (`self.PhysicResource`)))
    (set `self.SpeedDelayed` (`PFPhysicResource.GetForwardVelocityPercentage` (`self.PhysicResource`)))
    (else
      (`PFMathHelper.DecrementFloat` (`self.SpeedDelayed`) (* (`self.SpeedSlowSpeed`) (`local.deltaTime`)))))
  (`FMODBlueprintStatics.EventInstanceSetParameter` (`self.WindInstance`) "Speed" _returnvalue)
  (`FMODBlueprintStatics.EventInstanceSetParameter` (`self.MusicInstance`) "Speed" _returnvalue))