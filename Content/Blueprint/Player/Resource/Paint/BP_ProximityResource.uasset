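; Proximity paint component that finds paintable surfaces near a point offset in front of its owner.
; On each component tick or CheckCollisions event, it runs a zero-length multi sphere trace, skips landscapes and lazily initializes any BP_PaintableSurface it finds.
; Unique hits are stored alongside brush sizes remapped from their distance to the trace center; the painting itself is not done here.
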(event `self.ComponentTick`
  (params (deltaTime :type "Float (single-precision)"))
  (`self.CheckCollision`))

(event `self.CheckCollisions`
  (`self.CheckCollision`))

(fn `CheckCollision`
  (locals (StartPosition :type "Vector Structure") (Hit :type "HitResult Structure") (HitActor :type "Actor Object Reference"))
  (bind _owner (`self.Owner`))
  (bind (_x _y) (`KismetMathLibrary.BreakVector2D` (`self.BrushSizesMinMax`)))
  (bind _returnvalue (`Actor.GetComponentByClass` (`local.HitActor`) "/Game/Blueprint/Player/Resource/Paint/BP_PaintableSurface.BP_PaintableSurface_C"))
  (`KismetArrayLibrary.Array_Clear` (`self.ValidHitResults`))
  (`KismetArrayLibrary.Array_Clear` (`self.ValidBrushSizes`))
  (bind _output_get (set `local.StartPosition` (+ (`Actor.K2_GetActorLocation` _owner) (* (`Actor.GetActorForwardVector` _owner) (`self.BrushForwardOffset`)))))
  (bind _outhits (`KismetSystemLibrary.SphereTraceMulti` _output_get _output_get (`self.BrushSphereDistance`) "TraceTypeQuery1" true))
  (for _array_element _outhits
    (set `local.Hit` _array_element)
    (bind _output_get_2 (set `local.HitActor` (`.HitActor` (`GameplayStatics.BreakHitResult` _array_element))))
    (cast `Landscape` _output_get_2
      (:`CastFailed`
        (if (`KismetSystemLibrary.IsValid` _returnvalue)
          (if (not (`/Game/Blueprint/Player/Resource/Paint/BP_PaintableSurface.IsInnit` _returnvalue))
            (`/Game/Blueprint/Player/Resource/Paint/BP_PaintableSurface.InitPaintSurface` _returnvalue)
            (set `/Game/Blueprint/Player/Resource/Paint/BP_PaintableSurface.IsInnit` true _returnvalue))
          (bind _returnvalue_2 (`KismetArrayLibrary.Array_AddUnique` (`self.ValidHitResults`) (`local.Hit`)))
          (if (not (== _returnvalue_2 -1))
            (bind _returnvalue_3 (`PFMathHelper.RemapClamped` (`KismetMathLibrary.Vector_Distance` (`.ImpactPoint` (`GameplayStatics.BreakHitResult` (`local.Hit`))) (`local.StartPosition`)) (`self.BrushSphereDistance`) 0.0 _x _y))
            (`KismetArrayLibrary.Array_Add` (`self.ValidBrushSizes`) _returnvalue_3)))))))