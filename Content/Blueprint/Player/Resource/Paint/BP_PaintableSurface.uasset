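; Actor component that makes its owner's static mesh paintable at runtime through a render target.
; InitPaintSurface creates and clears the render target, feeds it to a dynamic instance of the mesh's first material, and creates a dynamic brush material.
; PaintBrush draws that brush material onto the render target at a normalized location, dividing brush size by the canvas material's BrushSize parameter.
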(event `self.ReceiveBeginPlay`
  (set `self.Mesh` (`Actor.GetComponentByClass` (`self.GetOwner`) "/Script/Engine.StaticMeshComponent")))

(fn `InitPaintSurface`
  (bind _texturesize (`self.TextureSize`))
  (if true
    (`|ExecutionSequence`
      (:`then_0`
        (bind _returnvalue (`KismetRenderingLibrary.CreateRenderTarget2D` _texturesize _texturesize))
        (bind _output_get (set `self.RenderTarget` _returnvalue))
        (`KismetRenderingLibrary.ClearRenderTarget2D` _output_get))
      (:`then_1`
        (bind _returnvalue_2 (`KismetMaterialLibrary.CreateDynamicMaterialInstance` (`PrimitiveComponent.GetMaterial` (`self.Mesh`) 0)))
        (bind _output_get_2 (set `self.materialCanvas` _returnvalue_2))
        (`MaterialInstanceDynamic.SetTextureParameterValue` _output_get_2 "RenderTarget" (`self.RenderTarget`))
        (`MaterialInstanceDynamic.SetTextureParameterValue` _returnvalue_2 "RenderTarget" (`self.RenderTarget`))
        (`PrimitiveComponent.SetMaterial` (`self.Mesh`) 0 _output_get_2))
      (:`then_2`
        (bind _returnvalue_3 (`KismetMaterialLibrary.CreateDynamicMaterialInstance` "/Game/TempArt/Material/PaintTest/M_/M_BrushPaint.M_BrushPaint"))
        (set `self.brushMat` _returnvalue_3)))))

(fn `PaintBrush`
  (params (BrushTexture :type "Texture2D Object Reference") (BrushSize :type "Float (double-precision)") (DrawLocation :type "Vector2D Structure"))
  (`|ExecutionSequence`
    (:`then_0`
      (`MaterialInstanceDynamic.SetTextureParameterValue` (`self.brushMat`) "BrushTexture" (`local.BrushTexture`)))
    (:`then_1`
      (bind (_canvas _size _context) (`KismetRenderingLibrary.BeginDrawCanvasToRenderTarget` (`self.RenderTarget`)))
      (bind _returnvalue (`MaterialInstanceDynamic.K2_GetScalarParameterValue` (`self.materialCanvas`) "BrushSize"))
      (bind _returnvalue_2 (/ (`local.BrushSize`) _returnvalue))
      (`Canvas.K2_DrawMaterial` _canvas (`self.brushMat`) (- (* _size (`local.DrawLocation`)) (/ _returnvalue_2 2.0)) (`KismetMathLibrary.MakeVector2D` _returnvalue_2 _returnvalue_2) (0.0 0.0) (1.0 1.0) 0.0 (0.5 0.5))
      (`KismetRenderingLibrary.EndDrawCanvasToRenderTarget` _context))))