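; Player paint resource that paints surfaces around its owner each tick through a painter, using hits from the proximity resource.
; Non-landscape hits need a BP_PaintableSurface, initialised on first use, and get brush sizes remapped by distance.
; Landscape painting uses a vertical trace ahead of the owner, sized by the nearest landscape proximity hit within range.
; That landscape pass also writes the owner's location to a material parameter collection.
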(event `self.ComponentInit`
  (params (ownerObj :type "PFPlayerCharacter Object Reference"))
  (`parent.ComponentInit` ownerObj)
  (bind _returnvalue (`PFPlayerCharacter.GetStateComponent` ownerObj "/Game/Blueprint/Player/Resource/Proximity/BP_ProximityResource.BP_ProximityResource_C"))
  (set `self.ProximityResource` _returnvalue)
  (bind _returnvalue_2 (`PFPlayerCharacter.GetStateComponent` ownerObj "/Game/Blueprint/Player/Resource/FlowerSpawner/BP_FlowerSpawnerResource.BP_FlowerSpawnerResource_C"))
  (set `self.FlowerResource` _returnvalue_2))

(event `self.ComponentTick`
  (params (deltaTime :type "Float (single-precision)"))
  (if (`KismetSystemLibrary.IsValid` (`self.ProximityResource`))
    (bind _returnvalue (`PFPainter.GetPainter` self))
    (bind (_validhitpaint1 _validbrushsizes1) (`self.FilterProximity`))
    (`PFPainter.PaintStuff` _returnvalue _validhitpaint1 _validbrushsizes1)
    (`self.LandscapePaint`)
    (else
      (`KismetSystemLibrary.PrintString` "[Paint Resource] the proximity resource reference is null, the floor will not be painted"))))

(fn `FilterProximity`
  (returns (ValidHitPaint1 :type "Array of HitResult Structure") (ValidBrushSizes1 :type "Array of Float (single-precision)"))
  (locals (ValidBrushSizes :type "Array of Float (single-precision)") (Hit :type "HitResult Structure") (HitActor :type "Actor Object Reference") (ValidHitPaint :type "Array of HitResult Structure"))
  (bind _returnvalue (`Actor.GetComponentByClass` (`local.HitActor`) "/Game/Blueprint/Player/Resource/Paint/BP_PaintableSurface.BP_PaintableSurface_C"))
  (bind (_brushsize_x _brushsize_y) (`KismetMathLibrary.BreakVector2D` (`PFPaintResourceData.BrushSize` (`self.PaintData`))))
  (for _array_element (`/Game/Blueprint/Player/Resource/Proximity/BP_ProximityResource.ValidHitResults` (`self.ProximityResource`))
    (set `local.Hit` _array_element)
    (bind _output_get (set `local.HitActor` (`.HitActor` (`GameplayStatics.BreakHitResult` _array_element))))
    (`/Engine/EditorBlueprintResources/StandardMacros.IsValid` _output_get
      (:`Is Valid`
        (cast `Landscape` _output_get
          (:`CastFailed`
            (if (`KismetSystemLibrary.IsValid` _returnvalue)
              (if (not (`/Game/Blueprint/Player/Resource/Paint/BP_PaintableSurface.IsInnit` _returnvalue))
                (`/Game/Blueprint/Player/Resource/Paint/BP_PaintableSurface.InitPaintSurface` _returnvalue)
                (set `/Game/Blueprint/Player/Resource/Paint/BP_PaintableSurface.IsInnit` true _returnvalue))
              (bind _returnvalue_2 (`KismetArrayLibrary.Array_AddUnique` (`local.ValidHitPaint`) (`local.Hit`)))
              (if (not (== _returnvalue_2 -1))
                (bind _returnvalue_3 (`PFMathHelper.RemapClamped` (`KismetMathLibrary.Vector_Distance` (`.ImpactPoint` (`GameplayStatics.BreakHitResult` (`local.Hit`))) (`Actor.K2_GetActorLocation` (`self.Owner`))) (`PFPaintResourceData.BrushMaxDistance` (`self.PaintData`)) 0.0 _brushsize_x _brushsize_y))
                (`KismetArrayLibrary.Array_Add` (`local.ValidBrushSizes`) _returnvalue_3))))))))
  (return (`local.ValidHitPaint`) (`local.ValidBrushSizes`)))

(fn `LandscapePaint`
  (locals (ClosestDist :type "Float (double-precision)"))
  (bind _owner (`self.Owner`))
  (bind _brushmaxdistancelandscape (`PFPaintResourceData.BrushMaxDistanceLandscape` (`self.PaintData`)))
  (bind (_brushsizelandscape_x _brushsizelandscape_y) (`KismetMathLibrary.BreakVector2D` (`PFPaintResourceData.BrushSizeLandscape` (`self.PaintData`))))
  (bind _returnvalue (+ (`Actor.K2_GetActorLocation` _owner) (* (`Actor.GetActorForwardVector` _owner) (`self.TraceForwardDistance`))))
  (bind (_outhit _returnvalue_2) (`KismetSystemLibrary.LineTraceSingle` (+ _returnvalue (0.0 0.0 -100000.0)) (+ _returnvalue (0.0 0.0 100000.0)) "TraceTypeQuery3" true))
  (if _returnvalue_2
    (set `local.ClosestDist` 100000000.0)
    (for _array_element (`/Game/Blueprint/Player/Resource/Proximity/BP_ProximityResource.ValidHitResults` (`self.ProximityResource`))
      (bind (_bblockinghit _binitialoverlap _time _distance _location _impactpoint _normal _impactnormal _physmat _hitactor) (`GameplayStatics.BreakHitResult` _array_element))
      (`/Engine/EditorBlueprintResources/StandardMacros.IsValid` _hitactor
        (:`Is Valid`
          (cast `Landscape` _hitactor)
          (bind _returnvalue_3 (`KismetMathLibrary.Vector_Distance` _impactpoint (`Actor.K2_GetActorLocation` (`self.Owner`))))
          (if (> (`local.ClosestDist`) _returnvalue_3)
            (set `local.ClosestDist` _returnvalue_3)))))
    (if (> _brushmaxdistancelandscape (`local.ClosestDist`))
      (bind _returnvalue_4 (`PFPainter.GetPainter` self))
      (bind _returnvalue_5 (`PFMathHelper.RemapClamped` (`local.ClosestDist`) _brushmaxdistancelandscape 0.0 _brushsizelandscape_x _brushsizelandscape_y))
      (`PFPainter.PaintStuff` _returnvalue_4 (`|MakeArray` _outhit) (`|MakeArray` _returnvalue_5))
      (`KismetMaterialLibrary.SetVectorParameterValue` "/Game/TempArt/Colorisation/MP_test.MP_test" "playerPos" (`KismetMathLibrary.Conv_VectorToLinearColor` (`Actor.K2_GetActorLocation` (`self.Owner`)))))
    (else
      (`KismetSystemLibrary.PrintString` "[PaintResource] No valid Hit" false true (struct :`R` 1.0 :`B` 0.031697 :`A` 1.0) 2.0 "PaintError"))))