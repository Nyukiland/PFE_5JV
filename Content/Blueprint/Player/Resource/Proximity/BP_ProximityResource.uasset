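; Player resource component that shows Niagara proximity effects when the player passes close to surfaces.
; Each tick it uses the closest hit to place and align either a water or dust effect, hiding both for misses or downward-facing surfaces.
; Forward velocity and hit distance drive effect parameters, while Landscape tag and slope select grass colors.
; An attenuated proximity haptics path is kept but never runs.
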(event `self.ComponentInit`
  (params (ownerObj :type "PFPlayerCharacter Object Reference"))
  (`parent.ComponentInit` ownerObj)
  (bind _returnvalue (`PFPlayerCharacter.GetStateComponent` (`self.Owner`) "/Game/Blueprint/Player/Resource/Haptics/BP_HapticsResource.BP_HapticsResource_C"))
  (set `self.HapticsResource` _returnvalue)
  (set `self.Timer` (`self.DurationAttenuation`))
  (bind _returnvalue_2 (`PFPlayerCharacter.GetStateComponent` (`self.Owner`) "/Game/Blueprint/Player/Resource/Physic/BP_PhysicResource.BP_PhysicResource_C"))
  (set `self.PhysicResource` _returnvalue_2)
  (`KismetSystemLibrary.DelayUntilNextTick`)
  (`KismetSystemLibrary.DelayUntilNextTick`)
  (`self.Deactivate` (`self.ProximityNiagara`)))

(event `self.ComponentTick`
  (params (deltaTime :type "Float (single-precision)"))
  (bind _output_get (set `self.Delta Time` deltaTime))
  (`parent.ComponentTick` _output_get)
  (`self.ProximityFeedback`))

(fn `ProximityFeedback`
  (bind _proximityniagarawater (`self.ProximityNiagaraWater`))
  (bind _proximityniagara (`self.ProximityNiagara`))
  (bind _returnvalue (`PFPhysicResource.GetForwardVelocityPercentage` (`self.PhysicResource`)))
  (bind (_bblockinghit _binitialoverlap _time _distance _location _impactpoint _normal _impactnormal) (`GameplayStatics.BreakHitResult` (`self.ClosestHitResult`)))
  (bind (_bblockinghit_2 _binitialoverlap_2 _time_2 _distance_2 _location_2 _impactpoint_2 _normal_2 _impactnormal_2 _physmat _hitactor) (`GameplayStatics.BreakHitResult` (`self.ClosestHitResult`)))
  (bind (_bblockinghit_3 _binitialoverlap_3 _time_3 _distance_3 _location_3 _impactpoint_3 _normal_3 _impactnormal_3) (`GameplayStatics.BreakHitResult` (`self.ClosestHitResult`)))
  (bind _returnvalue_2 (`PFPhysicResource.GetForwardVelocityPercentage` (`self.PhysicResource`)))
  (bind (_bblockinghit_4 _binitialoverlap_4 _time_4 _distance_4 _location_4 _impactpoint_4 _normal_4 _impactnormal_4) (`GameplayStatics.BreakHitResult` (`self.ClosestHitResult`)))
  (`/Engine/EditorBlueprintResources/StandardMacros.IsValid` (`self.ProximityNiagara`)
    (:`Is Valid`
      (if (and _bblockinghit (> (`KismetMathLibrary.Dot_VectorVector` _impactnormal (`KismetMathLibrary.Vector_Up`)) -0.35))
        (if (`Actor.ActorHasTag` (`.HitActor` (`GameplayStatics.BreakHitResult` (`self.ClosestHitResult`))) "Water")
          (if (not (`self.IsActive` (`self.ProximityNiagaraWater`)))
            (`self.Activate` (`self.ProximityNiagaraWater`) true)
            (`self.Deactivate` (`self.ProximityNiagara`)))
          ; Size
          (`NiagaraComponent.SetVariableFloat` (`self.ProximityNiagaraWater`) "Speed" (`KismetMathLibrary.Lerp` 500.0 2000.0 _returnvalue_2))
          (`NiagaraComponent.SetVariableFloat` (`self.ProximityNiagaraWater`) "Speed2" (`KismetMathLibrary.Lerp` 2000.0 5000.0 _returnvalue_2))
          (`NiagaraComponent.SetVariableFloat` (`self.ProximityNiagaraWater`) "Scale" (`KismetMathLibrary.Lerp` 1.0 4.0 _returnvalue_2))
          ; Position / Rotation
          (`SceneComponent.K2_SetWorldLocation` _proximityniagarawater (+ _impactpoint_4 (* _impactnormal_4 (100.0 100.0 100.0)) (* (`SceneComponent.GetForwardVector` (`self.ForwardRootPtr`)) (300.0 300.0 300.0))) false true)
          (`SceneComponent.K2_SetWorldRotation` _proximityniagarawater (`KismetMathLibrary.MakeRotFromXZ` (`Actor.GetActorForwardVector` (`self.Owner`)) (`.Normal` (`GameplayStatics.BreakHitResult` (`self.ClosestHitResult`)))) false true)
          (else
            (`self.Deactivate` (`self.ProximityNiagaraWater`))
            (if (not (`self.IsActive` (`self.ProximityNiagara`)))
              (`self.Activate` (`self.ProximityNiagara`) true))
            ; Size
            (`NiagaraComponent.SetVariableFloat` (`self.ProximityNiagara`) "Proximity" (- 1.0 (/ (`.Distance` (`GameplayStatics.BreakHitResult` (`self.ClosestHitResult`))) (`self.GetMaxClosestDistance`))))
            (`NiagaraComponent.SetVariableFloat` (`self.ProximityNiagara`) "ParticuleSpeed" (`KismetMathLibrary.Lerp` 1500.0 6000.0 _returnvalue))
            (`NiagaraComponent.SetVariableFloat` (`self.ProximityNiagara`) "Speed" _returnvalue)
            ; Position
            (`SceneComponent.K2_SetWorldLocation` _proximityniagara (+ _impactpoint_3 (* _impactnormal_3 (100.0 100.0 100.0)) (* (`SceneComponent.GetForwardVector` (`self.ForwardRootPtr`)) (300.0 300.0 300.0))) false true)
            (`SceneComponent.K2_SetWorldRotation` _proximityniagara (`KismetMathLibrary.MakeRotFromXZ` (`Actor.GetActorForwardVector` (`self.Owner`)) (`.Normal` (`GameplayStatics.BreakHitResult` (`self.ClosestHitResult`)))) false true)
            (`NiagaraComponent.SetVariableInt` (`self.ProximityNiagara`) "UseGrass" 0)
            ; Color
            (if (or (not (`Actor.ActorHasTag` _hitactor "Landscape")) (< (`KismetMathLibrary.Dot_VectorVector` _impactnormal_2 (`KismetMathLibrary.Vector_Up`)) 0.5))
              (`NiagaraComponent.SetVariableLinearColor` (`self.ProximityNiagara`) "DustColor" (`self.GroundColor`))
              (else
                (`NiagaraComponent.SetVariableLinearColor` (`self.ProximityNiagara`) "DustColor" (`self.GrassGroundColor`))
                (`NiagaraComponent.SetVariableLinearColor` (`self.ProximityNiagara`) "ParticleColor" (`self.GrassColor`))
                (`NiagaraComponent.SetVariableInt` (`self.ProximityNiagara`) "UseGrass" 1)))))
        (else
          (`self.Deactivate` (`self.ProximityNiagara`))
          (`self.Deactivate` (`self.ProximityNiagaraWater`)))))))