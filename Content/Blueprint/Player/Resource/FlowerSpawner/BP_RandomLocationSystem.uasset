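; Flower-spawning component that places BP_Flower actors from the owner's BP_ProximityResource hit data on a looping half-second timer.
; For each valid hit it traces from the owner and spawns a flower at the impact, aligned to the surface normal.
; The trace end uses only the hit normal, so the brush-sized random point goes unused.
; The time-seeded random-point helper is never called here.
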(event `self.ComponentInit`
  (params (ownerObj :type "PFPlayerCharacter Object Reference"))
  (set `self.Owner Obj` ownerObj)
  (`parent.ComponentInit` ownerObj)
  (bind _returnvalue (`PFPlayerCharacter.GetStateComponent` ownerObj "/Game/Blueprint/Player/Resource/Paint/BP_ProximityResource.BP_ProximityResource_C"))
  (set `self.ProximityResource` _returnvalue)
  (`KismetSystemLibrary.K2_SetTimerDelegate` (delegate `SpawnFlowerEvent`) 0.5 true))

(event `SpawnFlowerEvent`
  (`self.SpawnFlower`))

(event `self.ComponentEnable`)

(fn `FindRandomPointInBrushRadius`
  (params (Radius :type "Float (double-precision)"))
  (returns (RandomPointInBrushRadius :type "Vector2D Structure"))
  (locals (MinRangeValue :type "Float (double-precision)") (MaxRangeValue :type "Float (double-precision)") (XCoordonate :type "Float (double-precision)") (YCoordonate :type "Float (double-precision)"))
  (bind _output_get (set `local.MaxRangeValue` Radius))
  (set `local.MinRangeValue` (* _output_get -1.0))
  (bind _seed (`self.GetRandomSeed`))
  (set `local.XCoordonate` (`KismetMathLibrary.RandomFloatInRangeFromStream` _seed (`local.MinRangeValue`) (`local.MaxRangeValue`)))
  (bind _seed_2 (`self.GetRandomSeed`))
  (bind _output_get_2 (set `local.YCoordonate` (`KismetMathLibrary.RandomFloatInRangeFromStream` _seed_2 (`local.MinRangeValue`) (`local.MaxRangeValue`))))
  (return (`KismetMathLibrary.MakeVector2D` (`local.XCoordonate`) _output_get_2)))

(fn `GetRandomSeed`
  (returns (Seed :type "RandomStream Structure"))
  (return (`KismetMathLibrary.MakeRandomStream` (`KismetMathLibrary.FTrunc` (* (`GameplayStatics.GetTimeSeconds`) 100.0)))))

(fn `SpawnFlower`
  (for (_array_element _array_index) (`/Game/Blueprint/Player/Resource/Paint/BP_ProximityResource.ValidHitResults` (`self.ProximityResource`))
    ; Get random direction to spawn in the brush range (why should x radius by 15 ????)
    (`PFMathHelper.RandomPointInCircle` (* (`|GetArrayItem` (`/Game/Blueprint/Player/Resource/Proximity/BP_ProximityResource.ValidBrushSizes` (`self.ProximityResource`)) _array_index) 15.0))
    (bind (_returnvalue_x _returnvalue_y) (`KismetMathLibrary.BreakVector2D` (+ (0.0 0.0) (`KismetMathLibrary.MakeVector2D` (.x (`.ImpactNormal` (`GameplayStatics.BreakHitResult` _array_element))) (.y (`.ImpactNormal` (`GameplayStatics.BreakHitResult` _array_element)))))))
    ; Get normal and impact datas dor this point
    (bind _outhit (`KismetSystemLibrary.LineTraceSingle` (`Actor.K2_GetActorLocation` (`self.Owner Obj`)) (`KismetMathLibrary.MakeVector` _returnvalue_x _returnvalue_y (.z (`.ImpactNormal` (`GameplayStatics.BreakHitResult` _array_element)))) "TraceTypeQuery1" true))
    ; Spawn the flower
    (`|SpawnActorFromClass` "/Game/Blueprint/Vegetation/BP_Flower.BP_Flower_C" (`KismetMathLibrary.MakeTransform` (`.ImpactPoint` (`GameplayStatics.BreakHitResult` _outhit)) (`KismetMathLibrary.MakeRotFromZX` (`.ImpactNormal` (`GameplayStatics.BreakHitResult` _outhit)) (`KismetMathLibrary.Vector_Up`))) "AlwaysSpawn" "MultiplyWithRoot" null null)))