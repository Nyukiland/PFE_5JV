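; Player physics component that each tick runs pitch visuals, air friction, gravity and velocity processing, including angular, base max and override velocity.
; It then sphere-traces in place at the PhysicRoot's relative location and passes the hit to a white-circle material drawn into RT_test, which BeginPlay clears to black.
; The dynamic material is recreated every tick.
; A velocity debug print exists but never runs.
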(event `self.ReceiveBeginPlay`
  (`KismetRenderingLibrary.ClearRenderTarget2D` "/Game/TempArt/Colorisation/RT_test.RT_test"))

(event `self.ComponentTick`
  (params (deltaTime :type "Float (single-precision)"))
  (bind _relativelocation (`SceneComponent.RelativeLocation` (`self.PhysicRoot`)))
  (`parent.ComponentTick` deltaTime)
  (`self.ProcessPitchVisual` deltaTime)
  (`self.ProcessAirFriction` deltaTime)
  (`self.DoGravity` deltaTime)
  (`self.ProcessVelocity` deltaTime)
  (`self.ProcessBaseMaxVelocity` deltaTime)
  (`self.ProcessAngularVelocity` deltaTime)
  (`self.ProcessOverrideVelocity`)
  (bind _outhit (`KismetSystemLibrary.SphereTraceSingle` _relativelocation _relativelocation 300.0 "TraceTypeQuery1"))
  (set `self.positionHit` (`.Location` (`GameplayStatics.BreakHitResult` _outhit)))
  (bind _returnvalue (`KismetMaterialLibrary.CreateDynamicMaterialInstance` "/Game/TempArt/Colorisation/M_WhiteCircle.M_WhiteCircle"))
  (bind _output_get (set `self.dynMat` _returnvalue))
  (`MaterialInstanceDynamic.SetVectorParameterValue` _output_get "hitPosition" (`KismetMathLibrary.Conv_VectorToLinearColor` (`self.positionHit`)))
  (`KismetRenderingLibrary.DrawMaterialToRenderTarget` "/Game/TempArt/Colorisation/RT_test.RT_test" (`self.dynMat`)))

(fn `PrintDebug`
  (bind _currentglobalvelocity_ (`self.CurrentGlobalVelocity_`))
  (bind _currentforwardvelocity_ (`self.CurrentForwardVelocity_`))
  (`KismetSystemLibrary.PrintString` "[PhysicResource]")
  (`KismetSystemLibrary.PrintString` (`KismetStringLibrary.Concat_StrStr` "VelocityGlobal: " (`KismetStringLibrary.Conv_VectorToString` _currentglobalvelocity_) "/ Magnitude: " (`KismetStringLibrary.Conv_DoubleToString` (`KismetMathLibrary.VSize` _currentglobalvelocity_))))
  (`KismetSystemLibrary.PrintString` (`KismetStringLibrary.Concat_StrStr` "ForwardVelocity: " (`KismetStringLibrary.Conv_VectorToString` _currentforwardvelocity_) "/ Magnitude: " (`KismetStringLibrary.Conv_DoubleToString` (`KismetMathLibrary.VSize` _currentforwardvelocity_)))))