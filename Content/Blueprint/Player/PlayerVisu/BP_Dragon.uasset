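; BP_Dragon is a player visual Blueprint that drives the dragon's trail and drift effects through Niagara components.
; Each Tick, while its owner parent is valid, it reads values from a visual resource object.
; Alpha and speed line values feed two trail systems, and the drifting state activates or deactivates a speed sphere effect.
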(event `self.ReceiveTick`
  (params (DeltaSeconds :type "Float (single-precision)"))
  (`/Engine/EditorBlueprintResources/StandardMacros.IsValid` (`self.OwnerParentPtr`)
    (:`Is Valid`
      (`self.SetAlphaLine`)
      (`self.Set Speed Line`)
      (`self.SetDriftingFeedback`))))

(fn `Set Speed Line`
  (bind _value (`/Game/Blueprint/Player/Resource/Visual/BP_VisualResource.GetSpeedLineValue` (`self.VisualResourcePtr`)))
  (`NiagaraComponent.SetVariableFloat` (`self.NS_Trail`) "Speed" _value)
  (`NiagaraComponent.SetVariableFloat` (`self.NS_Trail1`) "Speed" _value))

(fn `SetAlphaLine`
  (bind _value (`/Game/Blueprint/Player/Resource/Visual/BP_VisualResource.GetAlphaLineValue` (`self.VisualResourcePtr`)))
  (`NiagaraComponent.SetVariableFloat` (`self.NS_Trail1`) "Alpha" _value)
  (`NiagaraComponent.SetVariableFloat` (`self.NS_Trail`) "Alpha" _value))

(fn `SetDriftingFeedback`
  (bind _ns_spherespeed (`self.NS_SphereSpeed`))
  (if (`/Game/Blueprint/Player/Resource/Visual/BP_VisualResource.GetDriftingState` (`self.VisualResourcePtr`))
    (`ActorComponent.Activate` _ns_spherespeed false)
    (else
      (`ActorComponent.Deactivate` _ns_spherespeed))))

(fn `UserConstructionScript`)