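; BP_Jet is a player visual Blueprint for the jet, turning movement state into mesh deformation and Niagara effects.
; SetOwnerParent caches the owner's dive and wingbeat ability components, whose values drive the Dive and Clap morph targets each tick.
; Tick also feeds line alpha and speed from VisualResourcePtr into two trail effects.
; The drifting state from VisualResourcePtr toggles the NSSphereSpeed effect.
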(event `self.ReceiveTick`
  (params (DeltaSeconds :type "Float (single-precision)"))
  (`/Engine/EditorBlueprintResources/StandardMacros.IsValid` (`self.OwnerParentPtr`)
    (:`Is Valid`
      (`self.SetAlphaLine`)
      (`self.Set Speed Line`)
      (`self.SetDriftingFeedback`)
      (bind _returnvalue (`PFDiveAbility.GetDivingValue` (`self.Dive`)))
      (`SkeletalMeshComponent.SetMorphTarget` (`self.jet`) "Dive" _returnvalue true)
      (bind _returnvalue_2 (`PFWingBeatAbility.GetCurrentWingBeatPercentage` (`self.WingBeat`)))
      (`SkeletalMeshComponent.SetMorphTarget` (`self.jet`) "Clap" _returnvalue_2 true))))

(fn `Set Speed Line`
  (bind _value (`/Game/Blueprint/Player/Resource/Visual/BP_VisualResource.GetSpeedLineValue` (`self.VisualResourcePtr`)))
  (`NiagaraComponent.SetVariableFloat` (`self.NS_Trail`) "Speed" _value)
  (`NiagaraComponent.SetVariableFloat` (`self.NS_Trail1`) "Speed" _value))

(fn `SetAlphaLine`
  (bind _value (`/Game/Blueprint/Player/Resource/Visual/BP_VisualResource.GetAlphaLineValue` (`self.VisualResourcePtr`)))
  (`NiagaraComponent.SetVariableFloat` (`self.NS_Trail1`) "Alpha" _value)
  (`NiagaraComponent.SetVariableFloat` (`self.NS_Trail`) "Alpha" _value))

(fn `SetDriftingFeedback`
  (bind _ns_spherespeed (`self.NS_SphereSpeed`))
  (if (`/Game/Blueprint/Player/Resource/Visual/BP_VisualResource.GetDriftingState` (`self.VisualResourcePtr`))
    (`ActorComponent.Activate` _ns_spherespeed false)
    (else
      (`ActorComponent.Deactivate` _ns_spherespeed))))

(fn `SetOwnerParent`
  (params (OwnerParentPtr :type "PFPlayerCharacter Object Reference"))
  (`parent.SetOwnerParent` OwnerParentPtr)
  (bind _returnvalue (`PFPlayerCharacter.GetStateComponent` (`self.OwnerParentPtr`) "/Game/Blueprint/Player/Ability/Dive/BP_DiveAbility.BP_DiveAbility_C"))
  (set `self.Dive` _returnvalue)
  (bind _returnvalue_2 (`PFPlayerCharacter.GetStateComponent` (`self.OwnerParentPtr`) "/Game/Blueprint/Player/Ability/WingBeat/BP_WingbeatAbility.BP_WingbeatAbility_C"))
  (set `self.WingBeat` _returnvalue_2))

(fn `UserConstructionScript`
  (`parent.UserConstructionScript`))