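; BP_TurnState is a player state that feeds left and right trigger input into turning.
; On each input event it stores the values and calls the parent handler first.
; For Triggered, Canceled and Completed events, it filters raw input by name and passes the X value to TurnPtr's left or right receive function.
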(event `self.OnInputTriggered`
  (params (inputName :type Name) (triggerEvent :type "ETriggerEvent Enum" :default "None") (value :type "InputActionValue Structure (by ref)"))
  (bind _trigger_event (`self.Trigger Event`))
  (bind _x (`EnhancedInputLibrary.BreakInputActionValue` (`self.InputValue`)))
  (set `self.Input Name` inputName)
  (set `self.Trigger Event` triggerEvent)
  (set `self.InputValue` value)
  (`parent.OnInputTriggered` (`self.Input Name`) (`self.Trigger Event`) (`self.InputValue`))
  (if (or (`|EnumEquality` _trigger_event "Triggered") (`|EnumEquality` _trigger_event "Canceled") (`|EnumEquality` _trigger_event "Completed"))
    (`PFBlueprintHelper.FilterAllInputRaw` (`self.Input Name`)
      (:`LeftTrigger`
        (`PFTurnAbility.ReceiveInputLeft` (`self.TurnPtr_`) _x))
      (:`RightTrigger`
        (`PFTurnAbility.ReceiveInputRight` (`self.TurnPtr_`) _x)))))