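; BP_WingBeatSubState is a player sub-state that turns the WingBeat input into a wing beat.
; It forwards every input event to the parent handler, then filters for the WingBeat input with a Triggered trigger.
; When the filter passes, it calls WingBeat on its WingBeatPtr reference.
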(event `self.OnInputTriggered`
  (params (inputName :type Name) (triggerEvent :type "ETriggerEvent Enum" :default "None") (value :type "InputActionValue Structure (by ref)"))
  (bind _trigger_event (`self.Trigger Event`))
  (set `self.Input Name` inputName)
  (set `self.Trigger Event` triggerEvent)
  (set `self.InputValue` value)
  (`parent.OnInputTriggered` (`self.Input Name`) _trigger_event (`self.InputValue`))
  (`PFBlueprintHelper.FilterSpecificInputWithTrigger` "WingBeat" "Triggered" (`self.Input Name`) _trigger_event
    (:`Passed`
      (`PFWingBeatAbility.WingBeat` (`self.WingBeatPtr_`)))))