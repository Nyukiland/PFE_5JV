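; BP_AutoDiveState is a player state that runs an automatic dive.
; On enter it adds a wing-beat substate and binds to that component's wing-beat event, while each tick advances the auto dive through the dive object.
; When a wing beat fires and the dive reports completion, the owner switches to BP_BaseCombinedState.
; Exiting unbinds the wing-beat event.
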(event `self.OnEnter`
  (`parent.OnEnter`)
  (`self.AddSubState` "/Game/Blueprint/Player/State/BP_WingBeatSubState.BP_WingBeatSubState_C")
  (add `PFWingBeatAbility.OnWingBeatCalled` (`self.WingBeatPtr_`) (delegate `ChangeState`)))

(event `ChangeState`
  (if (`PFDiveAbility.AutoDiveComplete` (`self.DivePtr_`))
    (`PFPlayerCharacter.ChangeState` (`self.Owner`) "/Game/Blueprint/Player/State/BP_BaseCombinedState.BP_BaseCombinedState_C")))

(event `self.OnTick`
  (params (deltaTime :type "Float (single-precision)"))
  (`parent.OnTick` deltaTime)
  (`PFDiveAbility.AutoDive` (`self.DivePtr_`) deltaTime))

(event `self.OnExit`
  (`parent.OnExit`)
  (clear `PFWingBeatAbility.OnWingBeatCalled` (`self.WingBeatPtr_`)))