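; BP_BaseCombinedState is a player state for gliding flight that combines several sub-states.
; On enter it adds sub-states for roll checking, turning, diving and wing beats.
; It filters Move input and forwards it to the glide object on triggered, canceled or completed events.
; Each tick it asks the glide object whether to auto-dive and, if so, switches the owner to BP_AutoDiveState.
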(event `self.OnEnter`
  (`parent.OnEnter`)
  (`self.AddSubState` "/Game/Blueprint/Player/State/BP_CheckRollSubState.BP_CheckRollSubState_C")
  (`self.AddSubState` "/Game/Blueprint/Player/State/BP_TurnSubState.BP_TurnSubState_C")
  (`self.AddSubState` "/Game/Blueprint/Player/State/BP_DiveSubState.BP_DiveSubState_C")
  (`self.AddSubState` "/Game/Blueprint/Player/State/BP_WingBeatSubState.BP_WingBeatSubState_C"))

(event `self.OnInputTriggered`
  (params (inputName :type Name) (triggerEvent :type "ETriggerEvent Enum" :default "None") (value :type "InputActionValue Structure (by ref)"))
  (bind (_x _y) (`EnhancedInputLibrary.BreakInputActionValue` (`self.InputValue`)))
  (set `self.Input Name` inputName)
  (set `self.Trigger Event` triggerEvent)
  (set `self.InputValue` value)
  (`parent.OnInputTriggered` (`self.Input Name`) (`self.Trigger Event`) (`self.InputValue`))
  (`PFBlueprintHelper.FilterSpecificInputRaw` "Move" (`self.Input Name`)
    (:`Passed`
      (`self.ReceiveMoveInput` (`KismetMathLibrary.MakeVector2D` _x _y)))))

(event `self.OnTick`
  (params (deltaTime :type "Float (single-precision)"))
  (`parent.OnTick` deltaTime)
  (`self.AutoDiveDetection`))

(fn `AutoDiveDetection`
  (bind _returnvalue (`PFGlideAbility.ShouldGoInAutoDive` (`self.GlidePtr_`)))
  (if _returnvalue
    (`PFPlayerCharacter.ChangeState` (`self.Owner`) "/Game/Blueprint/Player/State/BP_AutoDiveState.BP_AutoDiveState_C")))

(fn `ReceiveMoveInput`
  (params (Value :type "Vector2D Structure"))
  (locals (NewLocalVar :type Integer))
  (bind _trigger_event (`self.Trigger Event`))
  (if (or (`|EnumEquality` _trigger_event "Triggered") (`|EnumEquality` _trigger_event "Canceled") (`|EnumEquality` _trigger_event "Completed"))
    (`PFGlideAbility.ReceiveInputMovement` (`self.GlidePtr_`) Value)))