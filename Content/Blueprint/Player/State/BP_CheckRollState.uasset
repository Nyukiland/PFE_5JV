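; Player state that watches for left and right roll inputs and hands off to BP_RollState when a roll is confirmed.
; A roll input stores its direction and starts a timer; once it passes RollDelay, the state calls CallRoll and switches state.
; A wing beat cancels any pending roll and blocks new ones for RollDelay, separating the two actions.
; Setting the timer above its active threshold serves as the idle marker.
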(event `self.OnEnter`
  (`parent.OnEnter`)
  (set `self.TimerRoll` 11.0))

(event `self.OnInputTriggered`
  (params (inputName :type Name) (triggerEvent :type "ETriggerEvent Enum" :default "None") (value :type "InputActionValue Structure (by ref)"))
  (bind _returnvalue (`|EnumEquality` (`self.Trigger Event`) "Triggered"))
  (bind _returnvalue_2 (> (`self.WingBeatTimer`) (`self.RollDelay`)))
  (set `self.Trigger Event` triggerEvent)
  (set `self.InputValue` value)
  (`parent.OnInputTriggered` inputName (`self.Trigger Event`) (`self.InputValue`))
  (switch `name` inputName
    (:`IA_RollRight`
      (if _returnvalue
        (if _returnvalue_2
          (set `self.StoredRollValue` 1)
          (set `self.TimerRoll` 0.0))))
    (:`IA_RollLeft`
      (if _returnvalue
        (if _returnvalue_2
          (set `self.StoredRollValue` -1)
          (set `self.TimerRoll` 0.0))))
    (:`IA_WingBeat`
      (if (`|EnumEquality` (`self.Trigger Event`) "Triggered")
        (set `self.TimerRoll` 11.0)
        (set `self.WingBeatTimer` 0.0)))))

(event `self.OnTick`
  (params (deltaTime :type "Float (single-precision)"))
  (bind _output_get (set `self.Delta Time` deltaTime))
  (`parent.OnTick` _output_get)
  (`self.RollDetection` (`self.Delta Time`))
  (if (< (`self.WingBeatTimer`) (`self.RollDelay`))
    (`PFMathHelper.IncrementFloat` (`self.WingBeatTimer`) (`self.Delta Time`))))

(fn `RollDetection`
  (params (deltaTime :type "Float (double-precision)"))
  (if (< (`self.TimerRoll`) 10.0)
    (`PFMathHelper.IncrementFloat` (`self.TimerRoll`) deltaTime)
    (if (> (`self.TimerRoll`) (`self.RollDelay`))
      (`PFRollAbility.CallRoll` (`self.RollPtr_`) (`self.StoredRollValue`))
      (`PFPlayerCharacter.ChangeState` (`self.Owner`) "/Game/Blueprint/Player/State/BP_RollState.BP_RollState_C"))))