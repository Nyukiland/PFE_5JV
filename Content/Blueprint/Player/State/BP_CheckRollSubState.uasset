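; Player sub-state that watches for roll input and hands the owner over to the roll state.
; Left and right trigger inputs are filtered by name and forwarded to the roll object as roll attempts, each with its analog value and rotation side.
; Every tick it runs that object's pre-roll check and changes the owner's state to BP_RollState when the check passes.
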(event `self.OnEnter`
  (`parent.OnEnter`))

(event `self.OnInputTriggered`
  (params (inputName :type Name) (triggerEvent :type "ETriggerEvent Enum" :default "None") (value :type "InputActionValue Structure (by ref)"))
  (bind _inputvalue_x (break `InputActionValue` (`self.InputValue`)))
  (bind _inputvalue_x_2 (break `InputActionValue` (`self.InputValue`)))
  (set `self.Input Name` inputName)
  (set `self.Trigger Event` triggerEvent)
  (set `self.InputValue` value)
  (`PFBlueprintHelper.FilterSpecificInputRaw` "LeftTrigger" (`self.Input Name`)
    (:`Passed`
      (`PFRollAbility.TryCallRollLeft` (`self.RollPtr_`) _inputvalue_x_2 -1))
    (:`Blocked`
      (`PFBlueprintHelper.FilterSpecificInputRaw` "RightTrigger" (`self.Input Name`)
        (:`Passed`
          (`PFRollAbility.TryCallRollRight` (`self.RollPtr_`) _inputvalue_x 1))))))

(event `self.OnTick`
  (params (deltaTime :type "Float (single-precision)"))
  (bind _output_get (set `self.Delta Time` deltaTime))
  (`parent.OnTick` _output_get)
  (bind _returnvalue (`PFRollAbility.PreRollCheck` (`self.RollPtr_`) (`self.Delta Time`)))
  (if _returnvalue
    (`PFPlayerCharacter.ChangeState` (`self.Owner`) "/Game/Blueprint/Player/State/BP_RollState.BP_RollState_C")))