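; Player character for a bird flight game, hosting the pause, options and loading screen widgets, photo mode and unstuck recovery.
; BeginPlay wires scene components and Niagara effects into camera, visual, proximity, sound and physics resources, then freezes time during loading.
; Menus switch between pause and default states via time dilation; unstuck teleports to the spawn transform and relaunches forward.
; EndPlay exports collision playtest data to timestamped JSON.
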(event `self.ReceiveBeginPlay`
  (bind _root (`self.Root`))
  (set `self.safeTransform` (`KismetMathLibrary.MakeTransform` (`SceneComponent.K2_GetComponentLocation` _root) (`SceneComponent.K2_GetComponentRotation` _root) (`SceneComponent.K2_GetComponentScale` _root)))
  (`self.SetReferences`)
  (`parent.ReceiveBeginPlay`)
  (`FMODBlueprintStatics.VCASetVolume` "/Game/FMOD/VCAs/Master.Master")
  ; Pause
  (bind _returnvalue (`|CreateWidget` "/Game/Blueprint/UI/UW_Pause.UW_Pause_C" (`GameplayStatics.GetPlayerController` 0)))
  (set `self.PauseMenuRef` _returnvalue)
  (`UserWidget.AddToViewport` _returnvalue 0)
  (`/Game/Blueprint/UI/UW_Pause.Begin` _returnvalue self)
  (`Widget.SetVisibility` _returnvalue "Collapsed")
  ; Options
  (bind _returnvalue_2 (`|CreateWidget` "/Game/Blueprint/UI/UW_Options.UW_Options_C" (`GameplayStatics.GetPlayerController` 0)))
  (set `self.OptionMenuRef` _returnvalue_2)
  (`UserWidget.AddToViewport` _returnvalue_2 0)
  (`KismetSystemLibrary.DelayUntilNextTick`)
  (set `/Game/Blueprint/UI/UW_Options.Player Ref` self _returnvalue_2)
  (`/Game/Blueprint/UI/UW_Options.Begin` _returnvalue_2 true)
  (`Widget.SetVisibility` _returnvalue_2 "Collapsed")
  ; loading
  (bind _returnvalue_3 (`|CreateWidget` "/Game/Blueprint/UI/UW_LoadingScreen.UW_LoadingScreen_C" (`GameplayStatics.GetPlayerController` 0)))
  (set `self.LoadingScreenRef` _returnvalue_3)
  (`UserWidget.AddToViewport` _returnvalue_3 0)
  (`self.ChangeState` "/Game/Blueprint/Player/State/BP_PauseState.BP_PauseState_C")
  (`/Game/Blueprint/UI/UW_LoadingScreen.SetBar` _returnvalue_3)
  (`KismetSystemLibrary.Delay` 0.2)
  (`GameplayStatics.SetGlobalTimeDilation` 0.0)
  (`/Game/Blueprint/UI/UW_LoadingScreen.IsLoadingFinishedd` _returnvalue_3 self))

(event `CloseLoadingScreen`
  ; Menus
  (`GameplayStatics.SetGlobalTimeDilation` 1.0)
  (`KismetSystemLibrary.Delay` 2.0)
  (`FMODBlueprintStatics.VCASetVolume` "/Game/FMOD/VCAs/Master.Master" (/ (`/Game/Blueprint/UI/UW_Options.Master` (`self.OptionMenuRef`)) 10.0))
  (`Widget.RemoveFromParent` (`self.LoadingScreenRef`))
  (set `self.LoadingScreenRef` null)
  (`self.SetDefaultState`)
  (`PFPhysicResource.AddForwardVelocity` (`self.BP_PhysicResource`) 1000.0 true false 0.0 null))

(event `OpenOptions`
  (bind _optionmenuref (`self.OptionMenuRef`))
  ; Menus
  (`Widget.SetVisibility` _optionmenuref "Visible")
  (set `self.IsOptionOpen` true)
  (`/Game/Blueprint/UI/UW_Options.SendPlayerRefffff` _optionmenuref self)
  (`/Game/Blueprint/UI/UW_Options.Setup` _optionmenuref true))

(event `SetReferences`
  (bind _bp_cameraresource (`self.BP_CameraResource`))
  (`|ExecutionSequence`
    (:`then_0`
      (set `self.ForwardRootPtr` (`self.Forward_Root`))
      (set `self.PhysicRootPtr` (`self.Root`)))
    (:`then_1`
      (set `PFCameraResource.CameraPositionPtr_` (`self.CameraRoot`) _bp_cameraresource)
      (set `PFCameraResource.CameraPtr_` (`self.Kamela`) _bp_cameraresource)
      (set `PFCameraResource.CameraPitchPtr_` (`self.CameraPitch`) _bp_cameraresource)
      (set `PFCameraResource.CameraRollPtr_` (`self.CameraRoll`) _bp_cameraresource)
      (set `PFCameraResource.CameraYawPtr_` (`self.CameraYaw`) _bp_cameraresource))
    (:`then_2`
      (set `PFVisualResource.BirdVisualRootPtr_` (`self.BirdVisualContainer`) (`self.BP_VisualResource`))
      (`KismetSystemLibrary.DelayUntilNextTick`)
      (set `/Game/Blueprint/Player/Resource/Visual/BP_VisualResource.PetalNiagara` (`self.NS_Petals`) (`self.BP_VisualResource`))
      (set `/Game/Blueprint/Player/Resource/Visual/BP_VisualResource.WaterNiagara` (`self.NS_WaterBehindPlayer`) (`self.BP_VisualResource`))
      (set `/Game/Blueprint/Player/Resource/Proximity/BP_ProximityResource.ProximityNiagara` (`self.NS_Proximity`) (`self.BP_ProximityResource`))
      (set `/Game/Blueprint/Player/Resource/Proximity/BP_ProximityResource.ProximityNiagaraWater` (`self.NS_ProximityWater`) (`self.BP_ProximityResource`))
      (set `/Game/Blueprint/Player/Resource/Sound/BP_SoundResource.CaveSnapshot` (`self.Cave`) (`self.BP_SoundResource`)))))

(event `CloseOptions`
  (bind _optionmenuref (`self.OptionMenuRef`))
  ; Menus
  (`Widget.SetVisibility` _optionmenuref "Collapsed")
  (set `/Game/Blueprint/UI/UW_Options.IsMenuOpen` false _optionmenuref)
  (set `self.IsOptionOpen` false)
  (`self.OpenPause`))

(event `OpenPause`
  (bind _pausemenuref (`self.PauseMenuRef`))
  ; Menus
  (`Widget.SetVisibility` _pausemenuref "Visible")
  (set `/Game/Blueprint/UI/UW_Pause.IsMenuOpeeeeeen` true _pausemenuref)
  (`/Game/Blueprint/UI/UW_Pause.setup` _pausemenuref)
  (`self.ChangeState` "/Game/Blueprint/Player/State/BP_PauseState.BP_PauseState_C")
  (`GameplayStatics.SetGlobalTimeDilation` 0.0))

(event `ClosePause`
  (bind _pausemenuref (`self.PauseMenuRef`))
  (bind _optionmenuref (`self.OptionMenuRef`))
  ; Menus
  (`Widget.SetVisibility` _pausemenuref "Collapsed")
  (set `/Game/Blueprint/UI/UW_Pause.IsMenuOpeeeeeen` false _pausemenuref)
  (`self.SetDefaultState`)
  (`GameplayStatics.SetGlobalTimeDilation` 1.0)
  (if (`self.IsOptionOpen`)
    (`Widget.SetVisibility` _optionmenuref "Collapsed")
    (set `/Game/Blueprint/UI/UW_Options.IsMenuOpen` false _optionmenuref)
    (set `self.IsOptionOpen` false)))

(event `UnstuckCall`
  (bind _bp_physicresource (`self.BP_PhysicResource`))
  (bind (_safetransform_location _safetransform_rotation) (`KismetMathLibrary.BreakTransform` (`self.safeTransform`)))
  ; Menus
  (`SceneComponent.K2_SetWorldLocationAndRotation` (`self.Root`) _safetransform_location _safetransform_rotation false true)
  (`PFPhysicResource.StopAllMotion` _bp_physicresource true)
  (`PFPhysicResource.AddForwardVelocity` _bp_physicresource 1000.0 true false 0.0 null))

(event `EnhancedInput|/Game/Input/IA_Pause`
  (params (ActionValue :type Boolean) (ElapsedSeconds :type "Float (double-precision)") (TriggeredSeconds :type "Float (double-precision)") (InputAction :type "InputAction Object Reference" :default "/Game/Input/IA_Pause.IA_Pause"))
  (:`Started`
    (if (`/Game/Blueprint/UI/UW_Pause.IsMenuOpeeeeeen` (`self.PauseMenuRef`))
      (if (`self.IsOptionOpen`)
        (`self.CloseOptions`)
        (else
          (`self.ClosePause`)))
      (else
        (`self.OpenPause`)))))

(event `EnhancedInput|/Game/Input/IA_PhotoMode`
  (params (ActionValue :type Boolean) (ElapsedSeconds :type "Float (double-precision)") (TriggeredSeconds :type "Float (double-precision)") (InputAction :type "InputAction Object Reference" :default "/Game/Input/IA_PhotoMode.IA_PhotoMode"))
  (:`Triggered`
    (if (not (`/Game/Blueprint/UI/UW_Pause.IsMenuOpeeeeeen` (`self.PauseMenuRef`)))
      (bind _returnvalue (`|SpawnActorFromClass` "/Game/Blueprint/Player/BP_PhotoModePawn.BP_PhotoModePawn_C" (`SceneComponent.K2_GetComponentToWorld` (`self.Kamela`)) "Undefined" "MultiplyWithRoot" null null))
      (`/Game/Blueprint/Player/BP_PhotoModePawn.SetUp` _returnvalue self))))

(event `self.ReceiveEndPlay`
  (params (EndPlayReason :type "EEndPlayReason Enum" :default "Destroyed"))
  (bind (_year _month _day _hour _minute) (`KismetMathLibrary.BreakDateTime` (`KismetMathLibrary.Now`)))
  (`parent.ReceiveEndPlay` EndPlayReason)
  (bind _returnvalue (`GameplayStatics.GetCurrentLevelName` true))
  (`PFCollisionResource.ExportPlaytestDataToJson` (`self.BP_CollisionResource`) (`KismetStringLibrary.Concat_StrStr` _returnvalue "-" (`KismetSystemLibrary.GetPlatformUserName`) "(" (`KismetStringLibrary.Conv_IntToString` _day) "-" (`KismetStringLibrary.Conv_IntToString` _month) "-" (`KismetStringLibrary.Conv_IntToString` _hour) "-" (`KismetStringLibrary.Conv_IntToString` _minute) ")")))

(fn `UserConstructionScript`)