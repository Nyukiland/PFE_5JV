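; Bird ability component that drives the visual tilt of the bird model from left and right wing input.
; Each tick it runs the parent tick, ChangeRotation, then WingTurnVisual.
; WingTurnVisual lerps BirdVisual's relative pitch toward the signed input difference scaled by a data-driven max, using delta time and a data-driven rate.
; WingDiveVisual is an empty stub.
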(event `self.ComponentTick`
  (params (deltaTime :type "Float (single-precision)"))
  (`parent.ComponentTick` deltaTime)
  (`self.ChangeRotation` deltaTime)
  (`self.WingTurnVisual` deltaTime))

(fn `WingDiveVisual`)

(fn `WingTurnVisual`
  (params (deltaTime :type "Float (double-precision)"))
  (locals (RotValue :type "Float (double-precision)") (DTime :type "Float (double-precision)"))
  (bind _inputright_ (`self.InputRight_`))
  (bind _inputleft_ (`self.InputLeft_`))
  (bind (_relativerotation_roll _relativerotation_pitch _relativerotation_yaw) (`KismetMathLibrary.BreakRotator` (`SceneComponent.RelativeRotation` (`self.BirdVisual`))))
  (bind _returnvalue (- (`KismetMathLibrary.FMax` _inputright_ _inputleft_) (`KismetMathLibrary.FMin` _inputright_ _inputleft_)))
  (set `local.DTime` deltaTime)
  (if (> _inputright_ _inputleft_)
    (set `local.RotValue` _returnvalue)
    (else
      (set `local.RotValue` (* _returnvalue -1.0))))
  (`SceneComponent.K2_SetRelativeRotation` (`self.BirdVisual`) (`KismetMathLibrary.MakeRotator` _relativerotation_roll (`KismetMathLibrary.Lerp` _relativerotation_pitch (* (`PFWingVisualAbilityData.MaxRotationPitch` (`self.DataPtr_`)) (`local.RotValue`)) (* (`local.DTime`) (`PFWingVisualAbilityData.LerpWingRotation` (`self.DataPtr_`)))) _relativerotation_yaw) false false))