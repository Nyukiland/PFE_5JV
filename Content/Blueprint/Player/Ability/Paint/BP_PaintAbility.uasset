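; BP_PaintAbility is a player ability that paints onto surfaces around the actor as it moves through the world.
; Every tick, it runs a complex multi-sphere trace at the actor's location, with debug drawing on.
; It adds a PaintableLandscape component to hit landscapes or BP_PaintableSurface to other actors when missing.
; It then paints at each hit's collision UV, scaling brush size by impact distance.
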(event `self.ReceiveTick`
  (params (DeltaSeconds :type "Float (single-precision)"))
  (`self.CastToPaint_Sphere`))

(fn `CastToPaint_Sphere`
  (bind (_x _y) (`KismetMathLibrary.BreakVector2D` (`self.BrushSizeMinMax`)))
  (bind _returnvalue (`Actor.K2_GetActorLocation` (`self.Actor`)))
  (bind _outhits (`KismetSystemLibrary.SphereTraceMulti` :`Start` _returnvalue :`End` _returnvalue :`Radius` (`self.BrushSphereDistance`) :`TraceChannel` "TraceTypeQuery1" :`bTraceComplex` true :`DrawDebugType` "ForOneFrame"))
  (for _array_element _outhits
    (bind (_bblockinghit _binitialoverlap _time _distance _location _impactpoint _normal _impactnormal _physmat _hitactor) (`GameplayStatics.BreakHitResult` _array_element))
    (cast `Landscape` _hitactor
      (:`then`
        (if (not (`KismetSystemLibrary.IsValid` (`Actor.GetComponentByClass` _hitactor "/Game/TempArt/Material/PaintTest/PaintableLandscape.PaintableLandscape_C")))
          (`|AddComponentByClass` _hitactor "/Game/TempArt/Material/PaintTest/PaintableLandscape.PaintableLandscape_C"))
        (bind _uv (`GameplayStatics.FindCollisionUV` _array_element))
        (`/Game/TempArt/Material/PaintTest/PaintableLandscape.PaintBrush` (`Actor.GetComponentByClass` _hitactor "/Game/TempArt/Material/PaintTest/PaintableLandscape.PaintableLandscape_C") null (stale _returnvalue_2) _uv))
      (:`CastFailed`
        (if (not (`KismetSystemLibrary.IsValid` (`Actor.GetComponentByClass` _hitactor "/Game/Blueprint/Player/Ability/Paint/BP_PaintableSurface.BP_PaintableSurface_C")))
          (`|AddComponentByClass` _hitactor "/Game/Blueprint/Player/Ability/Paint/BP_PaintableSurface.BP_PaintableSurface_C"))
        (bind _returnvalue_2 (`PFMathHelper.RemapClamped` (`KismetMathLibrary.Vector_Distance` _impactpoint (`Actor.K2_GetActorLocation` (`self.Actor`))) (`self.BrushSphereDistance`) 0.0 _x _y))
        (`/Game/Blueprint/Player/Ability/Paint/BP_PaintableSurface.PaintBrush` (`Actor.GetComponentByClass` _hitactor "/Game/Blueprint/Player/Ability/Paint/BP_PaintableSurface.BP_PaintableSurface_C") "/Game/TempArt/Material/PaintTest/T_SineGradient007_-_transparent.T_SineGradient007_-_transparent" _returnvalue_2 _uv)))))