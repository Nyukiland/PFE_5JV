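; Actor component that makes its owner's static mesh paintable at runtime via render-target painting.
; On BeginPlay, if the slot 0 material's IsPaintable parameter is set, it creates a cleared render target, a dynamic canvas material that reads it, and a brush material instance.
; PaintBrush draws the supplied brush texture into that target at a normalized location, dividing brush size by the surface material's BrushSize parameter.
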(event `self.ReceiveBeginPlay`
  (set `self.Mesh` (`Actor.GetComponentByClass` (`self.GetOwner`) "/Script/Engine.StaticMeshComponent"))
  (`self.InitPaintSurface`))

(fn `InitPaintSurface`
  (bind _returnvalue (`KismetMaterialLibrary.CreateDynamicMaterialInstance` (`PrimitiveComponent.GetMaterial` (`self.Mesh`) 0) "None"))
  (bind _returnvalue_2 (`MaterialInstanceDynamic.K2_GetScalarParameterValue` _returnvalue "IsPaintable"))
  (if (> _returnvalue_2 0.0)
    (`|ExecutionSequence`
      (:`then_0`
        (bind _returnvalue_3 (`KismetRenderingLibrary.CreateRenderTarget2D` 1024 1024))
        (bind _output_get (set `self.RenderTarget` _returnvalue_3))
        (`KismetRenderingLibrary.ClearRenderTarget2D` _output_get))
      (:`then_1`
        (bind _returnvalue_4 (`KismetMaterialLibrary.CreateDynamicMaterialInstance` (`PrimitiveComponent.GetMaterial` (`self.Mesh`) 0)))
        (bind _output_get_2 (set `self.materialCanvas` _returnvalue_4))
        (`MaterialInstanceDynamic.SetTextureParameterValue` _returnvalue_4 "RenderTarget" (`self.RenderTarget`))
        (`MaterialInstanceDynamic.SetTextureParameterValue` _output_get_2 "RenderTarget" (`self.RenderTarget`))
        (`PrimitiveComponent.SetMaterial` (`self.Mesh`) 0 _output_get_2))
      (:`then_2`
        (bind _returnvalue_5 (`KismetMaterialLibrary.CreateDynamicMaterialInstance` "/Game/TempArt/Material/PaintTest/M_/M_BrushPaint.M_BrushPaint"))
        (set `self.brushMat` _returnvalue_5)))))

(fn `PaintBrush`
  (params (BrushTexture :type "Texture2D Object Reference") (BrushSize :type "Float (double-precision)") (DrawLocation :type "Vector2D Structure"))
  (bind _returnvalue (`MaterialInstanceDynamic.K2_GetScalarParameterValue` (`self.materialCanvas`) "IsPaintable"))
  (if (> _returnvalue 0.0)
    (`|ExecutionSequence`
      (:`then_0`
        (`MaterialInstanceDynamic.SetTextureParameterValue` (`self.brushMat`) "BrushTexture" (`local.BrushTexture`)))
      (:`then_1`
        (bind (_canvas _size _context) (`KismetRenderingLibrary.BeginDrawCanvasToRenderTarget` (`self.RenderTarget`)))
        (bind _returnvalue_2 (`MaterialInstanceDynamic.K2_GetScalarParameterValue` (`self.materialCanvas`) "BrushSize"))
        (bind _returnvalue_3 (/ (`local.BrushSize`) _returnvalue_2))
        (`Canvas.K2_DrawMaterial` _canvas (`self.brushMat`) (- (* _size (`local.DrawLocation`)) (/ _returnvalue_3 2.0)) (`KismetMathLibrary.MakeVector2D` _returnvalue_3 _returnvalue_3) (0.0 0.0) (1.0 1.0) 0.0 (0.5 0.5))
        (`KismetRenderingLibrary.EndDrawCanvasToRenderTarget` _context)))))