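; BP_DiveAbility is the player's dive ability component, adding speed-driven controller haptics on top of its parent's init and tick logic.
; On init it caches the owner's BP_HapticsResource state component.
; Each tick it samples CurveHaptics with the physics resource's forward velocity percentage and plays the result as the intensity of an open-ended "Dive" rumble on the large motors.
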(event `self.ComponentInit`
  (params (ownerObj :type "PFPlayerCharacter Object Reference"))
  (`parent.ComponentInit` ownerObj)
  (bind _returnvalue (`PFPlayerCharacter.GetStateComponent` (`self.Owner`) "/Game/Blueprint/Player/Resource/Haptics/BP_HapticsResource.BP_HapticsResource_C"))
  (set `self.HapticDive` _returnvalue))

(event `self.ComponentTick`
  (params (deltaTime :type "Float (single-precision)"))
  (`parent.ComponentTick` deltaTime)
  (`PFHapticsResource.PlayHaptics` (`self.HapticDive`) (`CurveFloat.GetFloatValue` (`self.curveHaptics`) (`PFPhysicResource.GetForwardVelocityPercentage` (`self.PhysicResourcePtr_`))) -1.0 "Dive" true false))