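; Free-flying camera pawn for photo mode, which takes control from the player and captures screenshots.
; Setup possesses the pawn, shows the photo UI, pauses the player's haptics and state machine, and makes their physics kinematic; closing reverses this and destroys the pawn.
; Inputs drive cine-camera-relative movement, trigger-based vertical motion and look.
; Taking a photo hides the UI for a tick during capture, guarded against re-entry.
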(event `SetUp`
  (params (Player :type "/Game/Blueprint/Player/BP_PlayerCharacter Object Reference"))
  (bind _returnvalue (`GameplayStatics.GetPlayerController` 0))
  (set `self.Player` Player)
  (`Controller.UnPossess` _returnvalue)
  (`KismetSystemLibrary.DelayUntilNextTick`)
  (`Controller.Possess` _returnvalue self)
  (bind _returnvalue_2 (`|CreateWidget` "/Game/Blueprint/UI/UW_PhotoUI.UW_PhotoUI_C"))
  (bind _output_get (set `self.UI` _returnvalue_2))
  (`UserWidget.AddToViewport` _output_get 0)
  (bind _returnvalue_3 (`PFPlayerCharacter.GetStateComponent` (`self.Player`) "/Game/Blueprint/Player/Resource/Haptics/BP_HapticsResource.BP_HapticsResource_C"))
  (`PFHapticsResource.AskToPauseHaptics` _returnvalue_3)
  (bind _returnvalue_4 (`PFPlayerCharacter.GetStateComponent` (`self.Player`) "/Game/Blueprint/Player/Resource/Physic/BP_PhysicResource.BP_PhysicResource_C"))
  (`PFPhysicResource.SetKinematic` _returnvalue_4 true)
  (`PFPlayerCharacter.SetStateMachineActiveState` (`self.Player`) false))

(event `EnhancedInput|/Game/Input/IA_ClosePause`
  (params (ActionValue :type Boolean) (ElapsedSeconds :type "Float (double-precision)") (TriggeredSeconds :type "Float (double-precision)") (InputAction :type "InputAction Object Reference" :default "/Game/Input/IA_ClosePause.IA_ClosePause"))
  (bind _returnvalue (`GameplayStatics.GetPlayerController` 0))
  (:`Triggered`
    (`Controller.UnPossess` _returnvalue :!label _label)
    (`KismetSystemLibrary.DelayUntilNextTick`)
    (`Controller.Possess` _returnvalue (`self.Player`))
    (`self.K2_DestroyActor`)
    (`Widget.RemoveFromParent` (`self.UI`))
    (set `self.UI` null)
    (bind _returnvalue_2 (`PFPlayerCharacter.GetStateComponent` (`self.Player`) "/Game/Blueprint/Player/Resource/Haptics/BP_HapticsResource.BP_HapticsResource_C"))
    (`PFHapticsResource.AskToResumeHaptics` _returnvalue_2)
    (bind _returnvalue_3 (`PFPlayerCharacter.GetStateComponent` (`self.Player`) "/Game/Blueprint/Player/Resource/Physic/BP_PhysicResource.BP_PhysicResource_C"))
    (`PFPhysicResource.SetKinematic` _returnvalue_3 false)
    (`PFPlayerCharacter.SetStateMachineActiveState` (`self.Player`) true)))

(event `EnhancedInput|/Game/Input/IA_PhotoMode`
  (params (ActionValue :type Boolean) (ElapsedSeconds :type "Float (double-precision)") (TriggeredSeconds :type "Float (double-precision)") (InputAction :type "InputAction Object Reference" :default "/Game/Input/IA_PhotoMode.IA_PhotoMode"))
  (:`Triggered`
    (goto _label)))

(event `EnhancedInput|/Game/Input/IA_Move`
  (params (ActionValue :type "Vector2D Structure") (ElapsedSeconds :type "Float (double-precision)") (TriggeredSeconds :type "Float (double-precision)") (InputAction :type "InputAction Object Reference" :default "/Game/Input/IA_Move.IA_Move"))
  (bind _cinecamera (`self.CineCamera`))
  (:`Triggered`
    (`self.AddMovementInput` (`SceneComponent.GetForwardVector` _cinecamera) ActionValue_Y)
    (`self.AddMovementInput` (`SceneComponent.GetRightVector` _cinecamera) ActionValue_X)))

(event `EnhancedInput|/Game/Input/IA_LeftTrigger`
  (params (ActionValue :type "Float (double-precision)") (ElapsedSeconds :type "Float (double-precision)") (TriggeredSeconds :type "Float (double-precision)") (InputAction :type "InputAction Object Reference" :default "/Game/Input/IA_LeftTrigger.IA_LeftTrigger"))
  (:`Triggered`
    (`self.AddMovementInput` (0.0 0.0 1.0) (* ActionValue -1.0))))

(event `EnhancedInput|/Game/Input/IA_RightTrigger`
  (params (ActionValue :type "Float (double-precision)") (ElapsedSeconds :type "Float (double-precision)") (TriggeredSeconds :type "Float (double-precision)") (InputAction :type "InputAction Object Reference" :default "/Game/Input/IA_RightTrigger.IA_RightTrigger"))
  (:`Triggered`
    (`self.AddMovementInput` (0.0 0.0 1.0) ActionValue)))

(event `EnhancedInput|/Game/Input/IA_Look`
  (params (ActionValue :type "Vector2D Structure") (ElapsedSeconds :type "Float (double-precision)") (TriggeredSeconds :type "Float (double-precision)") (InputAction :type "InputAction Object Reference" :default "/Game/Input/IA_Look.IA_Look"))
  (:`Triggered`
    (`self.AddControllerYawInput` ActionValue_X)
    (`self.AddControllerPitchInput` ActionValue_Y)))

(event `EnhancedInput|/Game/Input/IA_TakePhoto`
  (params (ActionValue :type Boolean) (ElapsedSeconds :type "Float (double-precision)") (TriggeredSeconds :type "Float (double-precision)") (InputAction :type "InputAction Object Reference" :default "/Game/Input/IA_TakePhoto.IA_TakePhoto"))
  (:`Triggered`
    (if (not (`self.Photo`))
      (set `self.Photo` true)
      (`Widget.SetVisibility` (`self.UI`) "Collapsed")
      (`KismetSystemLibrary.DelayUntilNextTick`)
      (`PFBlueprintHelper.CapturePhotoModeScreenshot`)
      (`Widget.SetVisibility` (`self.UI`) "Visible")
      (`KismetSystemLibrary.DelayUntilNextTick`)
      (set `self.Photo` false))))

(fn `UserConstructionScript`)