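; One-shot trigger behavior for an arch portal that spreads paint outward when the player crosses it.
; Crossing hides the portal, plays sound, haptics and a shockwave, then runs its linked actions.
; Tick grows a sphere trace over a timer, lazily initializing paintable surfaces, adds a vertical line-trace hit, and sends hits with brush sizes to the painter.
; Kill marks it crossed and starts painting without the feedback or actions.
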(event `self.OnTriggerEnter`
  (if (not (`self.IsCrossed`))
    (set `self.IsCrossed` true)
    (`SceneComponent.SetHiddenInGame` (`self.PortalVisual`) true false)
    (set `self.isPainting` true)
    (`FMODBlueprintStatics.PlayEventAtLocation` "/Game/FMOD/Events/Arch.Arch" (`Actor.GetTransform` (`self.GetOwner`)))
    (bind _returnvalue (`PFPlayerCharacter.GetStateComponent` (`PFTrigger.PlayerInTriggerPtr` (`self.TriggerObjectPtr_`)) "/Game/Blueprint/Player/Resource/Haptics/BP_HapticsResource.BP_HapticsResource_C"))
    (`PFHapticsResource.PlayHaptics` _returnvalue 0.5 1.5 "Arch" true true)
    (`SceneComponent.SetWorldScale3D` (`self.ShockWave`) (`KismetMathLibrary.Conv_DoubleToVector` (/ (`self.BrushSphereDistance`) 10000.0)))
    (`SceneComponent.K2_SetWorldLocation` (`self.ShockWave`) (`Actor.K2_GetActorLocation` (`PFTrigger.PlayerInTriggerPtr` (`self.TriggerObjectPtr_`))) false true)
    (`NiagaraComponent.ResetSystem` (`self.ShockWave`))
    (`self.Deactivate` (`self.Particules`))
    (for _array_element (`self.ActioToDo`)
      (`/Engine/EditorBlueprintResources/StandardMacros.IsValid` _array_element
        (:`Is Valid`
          (`/Game/Blueprint/LD/BP_ElementDoAction.DoAction` _array_element))))))

(event `Kill`
  (`SceneComponent.SetHiddenInGame` (`self.PortalVisual`) true false)
  (`SceneComponent.SetHiddenInGame` (`self.Particules`) true false)
  (set `self.IsCrossed` true)
  (set `self.isPainting` true))

(event `self.ReceiveTick`
  (params (DeltaSeconds :type "Float (single-precision)"))
  (if (`self.isPainting`)
    (bind _output_get (set `self.time` (+ DeltaSeconds (`self.time`))))
    (if (<= _output_get (`self.timer`))
      (bind (_validhitresultsref _brushsizesref) (`self.DetectCollisions`))
      (bind _returnvalue (`PFPainter.GetPainter` self))
      (`PFPainter.PaintStuff` _returnvalue _validhitresultsref _brushsizesref)
      (else
        (set `self.isPainting` false)))))

(fn `DetectCollisions`
  (returns (ValidHitResultsRef :type "Array of HitResult Structure") (BrushSizesRef :type "Array of Float (double-precision)"))
  (locals (ValidHitResults :type "Array of HitResult Structure") (ValidBrushSizes :type "Array of Float (double-precision)") (Hit :type "HitResult Structure") (HitActor :type "Actor Object Reference") (ClosestDist :type "Float (double-precision)"))
  (bind (_x _y) (`KismetMathLibrary.BreakVector2D` (`self.BrushSizeMinMax`)))
  (bind _returnvalue (`Actor.K2_GetActorLocation` (`self.GetOwner`)))
  (bind _returnvalue_2 (`Actor.K2_GetActorLocation` (`self.GetOwner`)))
  (bind (_x_2 _y_2) (`KismetMathLibrary.BreakVector2D` (`self.BrushSizeMinMax`)))
  (bind _returnvalue_3 (`Actor.GetComponentByClass` (`local.HitActor`) "/Game/Blueprint/Player/Resource/Paint/BP_PaintableSurface.BP_PaintableSurface_C"))
  (bind _returnvalue_4 (`KismetMathLibrary.Vector_Distance` (`.ImpactPoint` (`GameplayStatics.BreakHitResult` (`local.Hit`))) (`Actor.K2_GetActorLocation` (`self.GetOwner`))))
  (`KismetArrayLibrary.Array_Clear` (`local.ValidHitResults`))
  (`KismetArrayLibrary.Array_Clear` (`local.ValidBrushSizes`))
  (bind _outhits (`KismetSystemLibrary.SphereTraceMulti` _returnvalue _returnvalue (* (`self.BrushSphereDistance`) (/ (`self.time`) (`self.timer`))) "TraceTypeQuery5" true))
  (for _array_element _outhits
    (set `local.Hit` _array_element)
    (bind _output_get (set `local.HitActor` (`.HitActor` (`GameplayStatics.BreakHitResult` _array_element))))
    (cast `Landscape` _output_get
      (:`then`
        (if (> (`local.ClosestDist`) _returnvalue_4)
          (set `local.ClosestDist` _returnvalue_4)))
      (:`CastFailed`
        (if (`KismetSystemLibrary.IsValid` _returnvalue_3)
          (if (not (`/Game/Blueprint/Player/Resource/Paint/BP_PaintableSurface.IsInnit` _returnvalue_3))
            (`/Game/Blueprint/Player/Resource/Paint/BP_PaintableSurface.InitPaintSurface` _returnvalue_3)
            (set `/Game/Blueprint/Player/Resource/Paint/BP_PaintableSurface.IsInnit` true _returnvalue_3))
          (bind _returnvalue_5 (`KismetArrayLibrary.Array_AddUnique` (`local.ValidHitResults`) (`local.Hit`)))
          (if (not (== _returnvalue_5 -1))
            (bind _returnvalue_6 (`PFMathHelper.RemapClamped` (`KismetMathLibrary.Vector_Distance` (`.ImpactPoint` (`GameplayStatics.BreakHitResult` (`local.Hit`))) (`Actor.K2_GetActorLocation` (`self.GetOwner`))) (`self.BrushSphereDistance`) 0.0 _x_2 _y_2))
            (`KismetArrayLibrary.Array_Add` (`local.ValidBrushSizes`) _returnvalue_6))))))
  (bind (_outhit _returnvalue_7) (`KismetSystemLibrary.LineTraceSingle` (+ _returnvalue_2 (0.0 0.0 -100000.0)) (+ _returnvalue_2 (0.0 0.0 100000.0)) "TraceTypeQuery3" true))
  (if _returnvalue_7
    (bind _returnvalue_8 (`KismetArrayLibrary.Array_AddUnique` (`local.ValidHitResults`) _outhit))
    (if (not (== _returnvalue_8 -1))
      (`PFMathHelper.RemapClamped` (`local.ClosestDist`) (`self.BrushSphereDistance`) 0.0 _x _y)
      (`KismetArrayLibrary.Array_Add` (`local.ValidBrushSizes`) (* (/ (`self.BrushSphereDistance`) 10000.0) (* 300.0 (/ (`self.time`) (`self.timer`)))))
      (return (`local.ValidHitResults`) (`local.ValidBrushSizes`)))
    (else
      (return (`local.ValidHitResults`) (`local.ValidBrushSizes`)))))