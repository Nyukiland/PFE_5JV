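; BP_DirectionnalForceBehavior is a trigger behavior that pushes the player's physics with a set force while the trigger is active.
; Enter sets Active and refreshes the player's physics state component, but only if that pointer is already valid.
; Each tick adds Force as velocity with reset enabled.
; Exit clears Active and, when ExitForce is non-zero, calls AddVelocity with an end duration and curve, without passing ExitForce.
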(event `self.OnTriggerEnter`
  (set `self.bActive` true)
  (`/Engine/EditorBlueprintResources/StandardMacros.IsValid` (`self.PhysicPtr_`)
    (:`Is Valid`
      (bind _returnvalue (`PFPlayerCharacter.GetStateComponent` (`PFTrigger.PlayerInTriggerPtr` (`self.TriggerObjectPtr_`)) "/Script/PFE_5JV.PFPhysicResource"))
      (set `self.PhysicPtr_` _returnvalue))))

(event `self.OnTriggerExit`
  (set `self.bActive` false)
  (`/Engine/EditorBlueprintResources/StandardMacros.IsValid` (`self.PhysicPtr_`)
    (:`Is Valid`
      (if (!= (`self.ExitForce`) (0.0 0.0 0.0))
        (`PFPhysicResource.AddVelocity` (`self.PhysicPtr_`) (0.0 0.0 0.0) true false (`self.EndForceDuration`) (`self.EndForceCurbe`))))))

(event `self.OnTriggerTick`
  (params (deltaTime :type "Float (single-precision)"))
  (set `self.DeltaTime_` deltaTime)
  (if (`self.bActive`)
    (`/Engine/EditorBlueprintResources/StandardMacros.IsValid` (`self.PhysicPtr_`)
      (:`Is Valid`
        (`PFPhysicResource.AddVelocity` (`self.PhysicPtr_`) (`self.Force`) true false 0.0 null)))))