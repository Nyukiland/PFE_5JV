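; Trigger behavior that drives the forward velocity of the player inside a trigger volume.
; Entering activates it and, if the physics pointer is already valid, refreshes it from the player's BP_PhysicResource state component.
; While active, each tick overrides forward velocity with Force.
; Exiting deactivates it and adds a fixed forward velocity with the reset flag set.
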(event `self.OnTriggerEnter`
  (set `self.bActive` true)
  (`/Engine/EditorBlueprintResources/StandardMacros.IsValid` (`self.PhysicPtr_`)
    (:`Is Valid`
      (bind _returnvalue (`PFPlayerCharacter.GetStateComponent` (`PFTrigger.PlayerInTriggerPtr` (`self.TriggerObjectPtr_`)) "/Game/Blueprint/Player/Resource/Physic/BP_PhysicResource.BP_PhysicResource_C"))
      (set `self.PhysicPtr_` _returnvalue))))

(event `self.OnTriggerExit`
  (set `self.bActive` false)
  (`/Engine/EditorBlueprintResources/StandardMacros.IsValid` (`self.PhysicPtr_`)
    (:`Is Valid`
      (`PFPhysicResource.AddForwardVelocity` (`self.PhysicPtr_`) 300.0 true false 0.0 null))))

(event `self.OnTriggerTick`
  (params (deltaTime :type "Float (single-precision)"))
  (set `self.DeltaTime_` deltaTime)
  (if (`self.bActive`)
    (`/Engine/EditorBlueprintResources/StandardMacros.IsValid` (`self.PhysicPtr_`)
      (:`Is Valid`
        (`PFPhysicResource.OverrideForwardVelocity` (`self.PhysicPtr_`) (`self.Force`))))))