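; Trigger behavior for water volumes that puts the player in the reorientation state and restores the default state on exit.
; While inside, each tick reapplies that state and adds vertical velocity and pitch assist, scaled by a curve over elapsed time.
; An InWater counter on the collision resource gates dive and surfacing feedback: haptics and sound, plus flower color clearing on entry and water particles on exit.
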(event `self.OnTriggerEnter`
  (bind _returnvalue (`PFPlayerCharacter.GetStateComponent` (`PFTrigger.PlayerInTriggerPtr` (`self.TriggerObjectPtr_`)) "/Game/Blueprint/Player/Resource/Collsion/BP_CollisionResource.BP_CollisionResource_C"))
  (set `self.CollisionResourcePtr_` _returnvalue)
  (bind _returnvalue_2 (`PFPlayerCharacter.GetStateComponent` (`PFTrigger.PlayerInTriggerPtr` (`self.TriggerObjectPtr_`)) "/Game/Blueprint/Player/Resource/Physic/BP_PhysicResource.BP_PhysicResource_C"))
  (set `self.PhysicResourcePtr_` _returnvalue_2)
  (`PFPlayerCharacter.ChangeState` (`PFTrigger.PlayerInTriggerPtr` (`self.TriggerObjectPtr_`)) "/Game/Blueprint/Player/State/BP_ReorientationState.BP_ReorientationState_C")
  (`|ExecutionSequence`
    (:`then_0`
      (if (not (> (`/Game/Blueprint/Player/Resource/Collsion/BP_CollisionResource.InWater` (`self.CollisionResourcePtr_`)) 0))
        (bind _returnvalue_3 (`PFPlayerCharacter.GetStateComponent` (`PFTrigger.PlayerInTriggerPtr` (`self.TriggerObjectPtr_`)) "/Game/Blueprint/Player/Resource/Haptics/BP_HapticsResource.BP_HapticsResource_C"))
        (`PFHapticsResource.PlayHaptics` _returnvalue_3 0.8 -1.0 "Water" false true)
        (bind _returnvalue_4 (`PFPlayerCharacter.GetStateComponent` (`PFTrigger.PlayerInTriggerPtr` (`self.TriggerObjectPtr_`)) "/Game/Blueprint/Player/Resource/FlowerSpawner/BP_FlowerSpawnerResource.BP_FlowerSpawnerResource_C"))
        (`PFFlowerSpawnerResource.SetCurrentFlowerColor` _returnvalue_4 "EPFFC_None")
        (bind _returnvalue_5 (`PFPlayerCharacter.GetStateComponent` (`PFTrigger.PlayerInTriggerPtr` (`self.TriggerObjectPtr_`)) "/Game/Blueprint/Player/Resource/Sound/BP_SoundResource.BP_SoundResource_C"))
        (`/Game/Blueprint/Player/Resource/Sound/BP_SoundResource.CallDive` _returnvalue_5)))
    (:`then_1`
      (`PFMathHelper.IncrementInt` (`/Game/Blueprint/Player/Resource/Collsion/BP_CollisionResource.InWater` (`self.CollisionResourcePtr_`)) 1))))

(event `self.OnTriggerExit`
  (`PFMathHelper.DecrementInt` (`/Game/Blueprint/Player/Resource/Collsion/BP_CollisionResource.InWater` (`self.CollisionResourcePtr_`)) 1)
  (`PFMathHelper.ClampIntByRef` (`/Game/Blueprint/Player/Resource/Collsion/BP_CollisionResource.InWater` (`self.CollisionResourcePtr_`)) 0 1)
  (set `self.PhysicResourcePtr_` null)
  (`PFPlayerCharacter.SetDefaultState` (`PFTrigger.PlayerInTriggerPtr` (`self.TriggerObjectPtr_`)))
  (set `self.Timer` 0.0)
  (`|ExecutionSequence`
    (:`then_0`
      (if (<= (`/Game/Blueprint/Player/Resource/Collsion/BP_CollisionResource.InWater` (`self.CollisionResourcePtr_`)) 0)
        (bind _returnvalue (`PFPlayerCharacter.GetStateComponent` (`PFTrigger.PlayerInTriggerPtr` (`self.TriggerObjectPtr_`)) "/Game/Blueprint/Player/Resource/Haptics/BP_HapticsResource.BP_HapticsResource_C"))
        (`PFHapticsResource.PlayHaptics` _returnvalue 0.0 1.0 "Water" false true)
        (bind _returnvalue_2 (`PFPlayerCharacter.GetStateComponent` (`PFTrigger.PlayerInTriggerPtr` (`self.TriggerObjectPtr_`)) "/Game/Blueprint/Player/Resource/Visual/BP_VisualResource.BP_VisualResource_C"))
        (`/Game/Blueprint/Player/Resource/Visual/BP_VisualResource.CallWaterParticle` _returnvalue_2)
        (bind _returnvalue_3 (`PFPlayerCharacter.GetStateComponent` (`PFTrigger.PlayerInTriggerPtr` (`self.TriggerObjectPtr_`)) "/Game/Blueprint/Player/Resource/Sound/BP_SoundResource.BP_SoundResource_C"))
        (`/Game/Blueprint/Player/Resource/Sound/BP_SoundResource.CallDiveExit` _returnvalue_3)))
    (:`then_1`
      (set `self.CollisionResourcePtr_` null))))

(event `self.OnTriggerTick`
  (params (deltaTime :type "Float (single-precision)"))
  (bind _returnvalue (`CurveFloat.GetFloatValue` (`self.CurveForce`) (`KismetMathLibrary.FClamp` (/ (`self.Timer`) (`self.Duration`)))))
  (`PFPlayerCharacter.ChangeState` (`PFTrigger.PlayerInTriggerPtr` (`self.TriggerObjectPtr_`)) "/Game/Blueprint/Player/State/BP_ReorientationState.BP_ReorientationState_C")
  (`/Engine/EditorBlueprintResources/StandardMacros.IsValid` (`self.PhysicResourcePtr_`)
    (:`Is Valid`
      (`PFMathHelper.IncrementFloat` (`self.Timer`) deltaTime)
      (`PFPhysicResource.AddVelocity` (`self.PhysicResourcePtr_`) (`KismetMathLibrary.MakeVector` 0.0 0.0 (* _returnvalue (`self.UpForceInWater`))) true false 0.0 null)
      (`PFPhysicResource.AddAssistPitch` (`self.PhysicResourcePtr_`) (* _returnvalue (`self.PitchOffsetInWater`))))))