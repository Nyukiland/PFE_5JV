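; BP_CaveBehavior is a trigger behavior that switches cave ambiance for a player entering or leaving a trigger volume.
; On enter and exit it calls the parent handler, then fetches the BP_SoundResource state component from the player in the trigger.
; It passes a positive step on enter and a negative one on exit to SetCaveAmbiance, leaving the sound handling to that component.
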(event `self.OnTriggerEnter`
  (`parent.OnTriggerEnter`)
  (bind _returnvalue (`PFPlayerCharacter.GetStateComponent` (`PFTrigger.PlayerInTriggerPtr` (`self.TriggerObjectPtr_`)) "/Game/Blueprint/Player/Resource/Sound/BP_SoundResource.BP_SoundResource_C"))
  (`/Game/Blueprint/Player/Resource/Sound/BP_SoundResource.SetCaveAmbiance` _returnvalue 1))

(event `self.OnTriggerExit`
  (`parent.OnTriggerExit`)
  (bind _returnvalue (`PFPlayerCharacter.GetStateComponent` (`PFTrigger.PlayerInTriggerPtr` (`self.TriggerObjectPtr_`)) "/Game/Blueprint/Player/Resource/Sound/BP_SoundResource.BP_SoundResource_C"))
  (`/Game/Blueprint/Player/Resource/Sound/BP_SoundResource.SetCaveAmbiance` _returnvalue -1))