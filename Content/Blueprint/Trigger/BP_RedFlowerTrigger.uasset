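; BP_RedFlowerTrigger is a trigger that represents a red flower pickup, hosting a BP_BigFlower as a child actor.
; On begin play it sets that flower's color from the "B_Red" collection entry and feeds the returned color into the get-flower Niagara effect's particle color.
; When the trigger enter event fires, it restarts that effect and plays a sound.
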(event `self.ReceiveBeginPlay`
  (`parent.ReceiveBeginPlay`)
  (bind _asbp_big_flower (cast `/Game/Blueprint/Vegetation/BP_BigFlower` (`ChildActorComponent.ChildActor` (`self.BP_BigFlower`))))
  (bind _colorreturn (`/Game/Blueprint/Vegetation/BP_BigFlower.SetColorByCollectionName` _asbp_big_flower "B_Red"))
  (`NiagaraComponent.SetVariableLinearColor` (`self.NS_GetFlower`) "ParticleColor" _colorreturn))

(event `self.TriggerEnterEvent`
  (`NiagaraComponent.ResetSystem` (`self.NS_GetFlower`))
  (`FMODAudioComponent.Play` (`self.Sound`)))

(fn `UserConstructionScript`)