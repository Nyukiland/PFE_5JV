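; Arch trigger actor that sets up a portal arch by handing its visual and effect references to a BPBaseArcBehavior.
; On BeginPlay it passes in the portal visual, shockwave and particle effects, and sets the brush sphere distance from its Size value.
; The Blueprint holds no other logic: overlap and tick events are disabled stubs and the construction script is empty.
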(event `self.ReceiveBeginPlay`
  (set `/Game/Blueprint/Trigger/Behavior/BP_BaseArcBehavior.PortalVisual` (`self.PortalVisual`) (`self.BP_BaseArcBehavior`))
  (set `/Game/Blueprint/Trigger/Behavior/BP_BaseArcBehavior.ShockWave` (`self.VFX_Arch`) (`self.BP_BaseArcBehavior`))
  (set `/Game/Blueprint/Trigger/Behavior/BP_BaseArcBehavior.Particules` (`self.VFX_ArchParticule`) (`self.BP_BaseArcBehavior`))
  (set `/Game/Blueprint/Trigger/Behavior/BP_BaseArcBehavior.BrushSphereDistance` (`KismetMathLibrary.Conv_IntToDouble` (`self.Size`)) (`self.BP_BaseArcBehavior`)))

(fn `UserConstructionScript`)