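; Utility spline actor that lays a chosen static mesh along its spline as deformed, static, collidable spline mesh segments.
; The Rebuild event runs RebuildMesh, as the construction script is empty.
; RebuildMesh destroys SplineComponents on the actor's owner, not prior spline meshes, then adds segments matching spline position, tangent and scale.
; Segment count and segment length both come from spline length divided by Repetition, the count truncated.
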(event `Rebuild`
  (`self.RebuildMesh`))

(fn `RebuildMesh`
  (locals (length :type "Float (double-precision)"))
  (bind _spline (`self.Spline`))
  (bind _spline_2 (`self.Spline`))
  (bind _returnvalue (/ (`SplineComponent.GetSplineLength` (`self.Spline`)) (`KismetMathLibrary.Conv_IntToDouble` (`self.Repetition`))))
  (for _array_element (`self.K2_GetComponentsByClass` (`self.GetOwner`) "/Script/Engine.SplineComponent")
    (`ActorComponent.K2_DestroyComponent` _array_element))
  (`/Engine/EditorBlueprintResources/StandardMacros.IsValid` (`self.Mesh`)
    (:`Is Valid`
      (set `local.length` _returnvalue)
      (for _index (range (`KismetMathLibrary.FTrunc` _returnvalue))
        (bind _returnvalue_2 (`AddComponent|NODE_AddSplineMeshComponent-1`))
        (`SceneComponent.SetMobility` _returnvalue_2 "Static")
        (`StaticMeshComponent.SetStaticMesh` _returnvalue_2 (`self.Mesh`))
        (set `self.ForwardAxis` (`self.ForwardAxis`))
        (bind _returnvalue_3 (* _index (`local.length`)))
        (bind _returnvalue_4 (* (+ _index 1) (`local.length`)))
        (`SplineMeshComponent.SetStartAndEnd` _returnvalue_2 (`SplineComponent.GetLocationAtDistanceAlongSpline` _spline_2 _returnvalue_3 "Local") (* (`KismetMathLibrary.Normal` (`SplineComponent.GetTangentAtDistanceAlongSpline` _spline_2 _returnvalue_3 "Local")) (`local.length`)) (`SplineComponent.GetLocationAtDistanceAlongSpline` _spline _returnvalue_4 "Local") (* (`KismetMathLibrary.Normal` (`SplineComponent.GetTangentAtDistanceAlongSpline` _spline _returnvalue_4 "Local")) (`local.length`)) true)
        (bind (_returnvalue_x _returnvalue_y _returnvalue_z) (`KismetMathLibrary.BreakVector` (`SplineComponent.GetScaleAtDistanceAlongSpline` _spline_2 _returnvalue_3)))
        (`SplineMeshComponent.SetStartScale` _returnvalue_2 (`KismetMathLibrary.MakeVector2D` _returnvalue_y _returnvalue_z) true)
        (bind (_returnvalue_x_2 _returnvalue_y_2 _returnvalue_z_2) (`KismetMathLibrary.BreakVector` (`SplineComponent.GetScaleAtDistanceAlongSpline` _spline _returnvalue_4)))
        (`SplineMeshComponent.SetEndScale` _returnvalue_2 (`KismetMathLibrary.MakeVector2D` _returnvalue_y_2 _returnvalue_z_2) true)
        (`SceneComponent.K2_AttachToComponent` _returnvalue_2 (`self.Spline`) "None" "SnapToTarget" "SnapToTarget" "KeepRelative" true)
        (`PrimitiveComponent.SetCollisionEnabled` _returnvalue_2 "QueryAndPhysics")))))

(fn `UserConstructionScript`)