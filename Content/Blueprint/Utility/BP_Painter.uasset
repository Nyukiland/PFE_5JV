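; BP_Painter is a utility Blueprint that paints brush marks onto surfaces hit by traces.
; Its PaintStuff event takes hit results and per-hit brush sizes, skips Landscape actors, and requires a BP_PaintableSurface component on the hit actor.
; It initializes each surface on first use, then stamps a fixed gradient brush texture at the hit's collision UV using the matching brush size.
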(event `self.PaintStuff`
  (params (validHitResults :type "Array of HitResult Structure (by ref)") (brushSizes :type "Array of Float (single-precision) (by ref)"))
  (`self.ApplyTextures` validHitResults brushSizes))

(fn `ApplyTextures`
  (params (ValidHitResults :type "Array of HitResult Structure") (BrushSizes :type "Array of Float (double-precision)"))
  (locals (Index :type Integer))
  (for (_array_element _array_index) ValidHitResults
    (set `local.Index` _array_index)
    (bind (_bblockinghit _binitialoverlap _time _distance _location _impactpoint _normal _impactnormal _physmat _hitactor) (`GameplayStatics.BreakHitResult` _array_element))
    (cast `Landscape` _hitactor
      (:`CastFailed`
        (bind _returnvalue (`self.GetComponentByClass` _hitactor "/Game/Blueprint/Player/Resource/Paint/BP_PaintableSurface.BP_PaintableSurface_C"))
        (if (`KismetSystemLibrary.IsValid` _returnvalue)
          (if (not (`/Game/Blueprint/Player/Resource/Paint/BP_PaintableSurface.IsInnit` _returnvalue))
            (`/Game/Blueprint/Player/Resource/Paint/BP_PaintableSurface.InitPaintSurface` _returnvalue)
            (set `/Game/Blueprint/Player/Resource/Paint/BP_PaintableSurface.IsInnit` true _returnvalue))
          (`/Game/Blueprint/Player/Resource/Paint/BP_PaintableSurface.PaintBrush` _returnvalue "/Game/TempArt/Material/PaintTest/T_SineGradient007_-_transparent.T_SineGradient007_-_transparent" (`|GetArrayItem` (`local.BrushSizes`) (`local.Index`)) (`GameplayStatics.FindCollisionUV` (`|GetArrayItem` (`local.ValidHitResults`) (`local.Index`)))))))))

(fn `UserConstructionScript`)