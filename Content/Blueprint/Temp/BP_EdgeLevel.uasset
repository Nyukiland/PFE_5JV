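; BP_EdgeLevel is a level-edge actor that fades a post-process effect in and out as the player crosses its trigger.
; EdgeTrigger toggles IsOutside on each player overlap, while the safety volumes always clear it and run the fade-out.
; Timeline and Exit drive both PostProcess.BlendWeight and the EdgeBlend collection parameter.
; Each timeline's start time is seeded from the current weight, so reversals avoid restarting the blend.
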(event `self.EdgeTrigger.OnComponentBeginOverlap`
  (params (OverlappedComponent :type "PrimitiveComponent Object Reference") (OtherActor :type "Actor Object Reference") (OtherComp :type "PrimitiveComponent Object Reference") (OtherBodyIndex :type Integer) (bFromSweep :type Boolean) (SweepResult :type "HitResult Structure (by ref)"))
  (cast `/Game/Blueprint/Player/BP_PlayerCharacter` OtherActor)
  (if (not (`self.isOutside`))
    (set `self.isOutside` true)
    (`|ExecutionSequence`
      (:`then_0`
        (bind (_direction _blend) (`Timeline|Timeline` :`NewTime` (`PostProcessComponent.BlendWeight` (`self.PostProcess`)) :!via `SetNewTime` :!label _label)
          (:`Update`
            (`KismetMaterialLibrary.SetScalarParameterValue` "/Game/Materials/POST_PROCESS/MParameter_PostPro.MParameter_PostPro" "EdgeBlend" _blend)
            (set `PostProcessComponent.BlendWeight` _blend (`self.PostProcess`)))))
      (:`then_1`
        (goto _label)))
    (else
      (set `self.isOutside` false :!label _label_2)
      (`|ExecutionSequence`
        (:`then_0`
          (bind (_direction_2 _blend_2) (`Timeline|Exit` :`NewTime` (- 1.0 (`PostProcessComponent.BlendWeight` (`self.PostProcess`))) :!via `SetNewTime` :!label _label_3)
            (:`Update`
              (`KismetMaterialLibrary.SetScalarParameterValue` "/Game/Materials/POST_PROCESS/MParameter_PostPro.MParameter_PostPro" "EdgeBlend" _blend_2)
              (set `PostProcessComponent.BlendWeight` _blend_2 (`self.PostProcess`)))))
        (:`then_1`
          (goto _label_3))))))

(event `self.EdgeTriggerSafety.OnComponentBeginOverlap`
  (params (OverlappedComponent :type "PrimitiveComponent Object Reference") (OtherActor :type "Actor Object Reference") (OtherComp :type "PrimitiveComponent Object Reference") (OtherBodyIndex :type Integer) (bFromSweep :type Boolean) (SweepResult :type "HitResult Structure (by ref)"))
  (cast `/Game/Blueprint/Player/BP_PlayerCharacter` OtherActor :!label _label_4)
  (goto _label_2))

(event `self.BoxSafety.OnComponentBeginOverlap`
  (params (OverlappedComponent :type "PrimitiveComponent Object Reference") (OtherActor :type "Actor Object Reference") (OtherComp :type "PrimitiveComponent Object Reference") (OtherBodyIndex :type Integer) (bFromSweep :type Boolean) (SweepResult :type "HitResult Structure (by ref)"))
  (goto _label_4))

(event `self.BoxSafety1.OnComponentBeginOverlap`
  (params (OverlappedComponent :type "PrimitiveComponent Object Reference") (OtherActor :type "Actor Object Reference") (OtherComp :type "PrimitiveComponent Object Reference") (OtherBodyIndex :type Integer) (bFromSweep :type Boolean) (SweepResult :type "HitResult Structure (by ref)"))
  (goto _label_4))

(event `self.BoxSafety2.OnComponentBeginOverlap`
  (params (OverlappedComponent :type "PrimitiveComponent Object Reference") (OtherActor :type "Actor Object Reference") (OtherComp :type "PrimitiveComponent Object Reference") (OtherBodyIndex :type Integer) (bFromSweep :type Boolean) (SweepResult :type "HitResult Structure (by ref)"))
  (goto _label_4))

(event `self.BoxSafety3.OnComponentBeginOverlap`
  (params (OverlappedComponent :type "PrimitiveComponent Object Reference") (OtherActor :type "Actor Object Reference") (OtherComp :type "PrimitiveComponent Object Reference") (OtherBodyIndex :type Integer) (bFromSweep :type Boolean) (SweepResult :type "HitResult Structure (by ref)"))
  (goto _label_4))

(fn `UserConstructionScript`)