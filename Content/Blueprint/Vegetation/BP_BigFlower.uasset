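; BP_BigFlower is a big flower vegetation Blueprint with a mesh, light cone, point light and Niagara particle effect.
; SetColorByCollectionName reads a named vector from the FlowerColorCollection parameter collection, applies it to all four components as one shared color, and returns it.
; The particle system resets on BeginPlay, and nothing in this graph calls the color function itself.
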(event `self.ReceiveBeginPlay`
  (`NiagaraComponent.ResetSystem` (`self.NS_FlowerParticules`)))

(fn `SetColorByCollectionName`
  (params (CollectionName :type Name))
  (returns (ColorReturn :type "LinearColor Structure"))
  (bind _returnvalue (`KismetMaterialLibrary.GetVectorParameterValue` (`self.Flower Color Collection`) CollectionName))
  (`MeshComponent.SetColorParameterValueOnMaterials` (`self.M_BigFlower_02`) "FlowerColor" _returnvalue)
  (`MeshComponent.SetColorParameterValueOnMaterials` (`self.LightCone`) "Color" _returnvalue)
  (`LightComponent.SetLightColor` (`self.PointLight`) _returnvalue true)
  (`NiagaraComponent.SetVariableLinearColor` (`self.NS_FlowerParticules`) "ParticleColor" _returnvalue)
  (return _returnvalue))

(fn `UserConstructionScript`)