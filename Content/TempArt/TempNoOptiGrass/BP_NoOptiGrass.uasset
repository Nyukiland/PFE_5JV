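; BP_NoOptiGrass is a temporary, unoptimized grass patch that animates to life when the player enters its sphere trigger.
; BeginPlay creates one dynamic M_GrassNoOpti material instance and shares it across all its static meshes.
; The first BP_PlayerCharacter overlap starts a one-shot, self-calling next-tick loop.
; The loop accumulates the delta time cached by Tick, ramping the Alive material parameter up to one.
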(event `self.ReceiveBeginPlay`
  (bind _returnvalue (`PrimitiveComponent.CreateDynamicMaterialInstance` (`self.StaticMesh`) 0 "/Game/TempArt/TempNoOptiGrass/M_GrassNoOpti.M_GrassNoOpti" "None"))
  (bind _output_get (set `self.Material` _returnvalue))
  (`PrimitiveComponent.SetMaterial` (`self.StaticMesh2`) 0 _output_get)
  (`PrimitiveComponent.SetMaterial` (`self.StaticMesh1`) 0 _output_get)
  (`PrimitiveComponent.SetMaterial` (`self.StaticMesh3`) 0 _output_get)
  (`PrimitiveComponent.SetMaterial` (`self.StaticMesh4`) 0 _output_get)
  (`PrimitiveComponent.SetMaterial` (`self.StaticMesh5`) 0 _output_get)
  (`PrimitiveComponent.SetMaterial` (`self.StaticMesh6`) 0 _output_get)
  (`PrimitiveComponent.SetMaterial` (`self.StaticMesh7`) 0 _output_get)
  (`PrimitiveComponent.SetMaterial` (`self.StaticMesh8`) 0 _output_get)
  (`PrimitiveComponent.SetMaterial` (`self.StaticMesh9`) 0 _output_get)
  (`PrimitiveComponent.SetMaterial` (`self.StaticMesh10`) 0 _output_get)
  (`PrimitiveComponent.SetMaterial` (`self.StaticMesh11`) 0 _output_get))

(event `self.ReceiveTick`
  (params (DeltaSeconds :type "Float (single-precision)"))
  (set `self.Delta Seconds` DeltaSeconds))

(event `self.Sphere.OnComponentBeginOverlap`
  (params (OverlappedComponent :type "PrimitiveComponent Object Reference") (OtherActor :type "Actor Object Reference") (OtherComp :type "PrimitiveComponent Object Reference") (OtherBodyIndex :type Integer) (bFromSweep :type Boolean) (SweepResult :type "HitResult Structure (by ref)"))
  (cast `/Game/Blueprint/Player/BP_PlayerCharacter` OtherActor)
  (if (not (`self.DoOnce`))
    (set `self.DoOnce` true)
    (`self.Custom Loop`)))

(event `Custom Loop`
  (if (not (>= (`self.lerpValue`) 1.0))
    (bind _returnvalue (`PFMathHelper.IncrementFloat` (`self.lerpValue`) (`self.Delta Seconds`)))
    (bind _output_get (set `self.lerpValue` (`KismetMathLibrary.FClamp` _returnvalue)))
    (`MaterialInstanceDynamic.SetScalarParameterValue` (`self.Material`) "Alive" _output_get)
    (`KismetSystemLibrary.DelayUntilNextTick`)
    (`self.Custom Loop`)))

(fn `UserConstructionScript`)