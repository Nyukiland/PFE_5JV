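; BP_RVTtester is a test Blueprint that paints on paintable surfaces, apparently for trying out RVT landscape painting.
; Every Tick it fires a complex line trace straight up from its location, with a one-frame debug line.
; When the hit actor has a BP_PaintableSurface component, it gets the painter and passes the hit to PaintStuff, using Scale as the brush size.
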(event `self.ReceiveActorBeginOverlap`
  (params (OtherActor :type "Actor Object Reference")))

(event `self.ReceiveBeginPlay`)

(event `self.ReceiveTick`
  (params (DeltaSeconds :type "Float (single-precision)"))
  (bind _returnvalue (`self.K2_GetActorLocation` self))
  (bind (_outhit _returnvalue_2) (`KismetSystemLibrary.LineTraceSingle` :`Start` _returnvalue :`End` (+ _returnvalue (0.0 0.0 10000000.0)) :`TraceChannel` "TraceTypeQuery3" :`bTraceComplex` true :`DrawDebugType` "ForOneFrame"))
  (if _returnvalue_2
    (if (`KismetSystemLibrary.IsValid` (`self.GetComponentByClass` (`.HitActor` (`GameplayStatics.BreakHitResult` _outhit)) "/Game/Blueprint/Player/Resource/Paint/BP_PaintableSurface.BP_PaintableSurface_C"))
      (bind _returnvalue_3 (`PFPainter.GetPainter` self))
      (`PFPainter.PaintStuff` _returnvalue_3 (`|MakeArray` _outhit) (`|MakeArray` (`self.scale`) :!type "Float (single-precision)")))))

(fn `UserConstructionScript`)