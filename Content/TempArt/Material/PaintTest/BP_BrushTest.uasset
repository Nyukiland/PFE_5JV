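; BP_BrushTest is a test actor that paints onto surfaces around it.
; Each Tick it runs a complex multi sphere trace at its location, with debug drawing, and adds a BP_PaintableSurface component to hit actors lacking one.
; It then calls PaintBrush on that component with a gradient texture at the hit's collision UV, sizing the brush by distance to the impact point.
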(event `self.ReceiveTick`
  (params (DeltaSeconds :type "Float (single-precision)"))
  (`self.CastToPaint_Sphere`))

(fn `CastToPaint_Sphere`
  (bind (_x _y) (`KismetMathLibrary.BreakVector2D` (`self.BrushSize`)))
  (bind _returnvalue (`self.K2_GetActorLocation` self))
  (bind _outhits (`KismetSystemLibrary.SphereTraceMulti` :`Start` _returnvalue :`End` _returnvalue :`Radius` (`self.Distance`) :`TraceChannel` "TraceTypeQuery1" :`bTraceComplex` true :`DrawDebugType` "ForOneFrame"))
  (for _array_element _outhits
    (bind (_bblockinghit _binitialoverlap _time _distance _location _impactpoint _normal _impactnormal _physmat _hitactor) (`GameplayStatics.BreakHitResult` _array_element))
    (if (not (`KismetSystemLibrary.IsValid` (`self.GetComponentByClass` _hitactor "/Game/Blueprint/Player/Resource/Paint/BP_PaintableSurface.BP_PaintableSurface_C")))
      (`AddComponent|NODE_AddPaintableSurface-0` :`self` _hitactor))
    (bind _returnvalue_2 (`PFMathHelper.RemapClamped` (`KismetMathLibrary.Vector_Distance` _impactpoint (`self.K2_GetActorLocation` self)) (`self.Distance`) 0.0 _x _y))
    (`/Game/Blueprint/Player/Resource/Paint/BP_PaintableSurface.PaintBrush` (`self.GetComponentByClass` _hitactor "/Game/Blueprint/Player/Resource/Paint/BP_PaintableSurface.BP_PaintableSurface_C") "/Game/TempArt/Material/PaintTest/T_SineGradient007_-_transparent.T_SineGradient007_-_transparent" _returnvalue_2 (`GameplayStatics.FindCollisionUV` _array_element))))

(fn `UserConstructionScript`)